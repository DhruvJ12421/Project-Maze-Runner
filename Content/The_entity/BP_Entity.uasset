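; Hostile entity actor that chases the player, draining health and applying glitch effects at close range.
; Tick moves it by unswept world offset toward the player or a target door's look spot.
; Looping timers trace for doors and check whether the player is home, switching the target to the nearest BP_HomeDoor and toggling particle visibility.
; SetInactive parks it underground; SetActive teleports it to a random distant point around the player.
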(event Custom|Check%20for%20Door
  (bind _returnvalue (Transformation|GetActorLocation))
  ;[1 1 1] checks if door infront of it is closed or not
  (bind _outhits (Collision|MultiLineTraceByChannel _returnvalue (+ _returnvalue (* (Transformation|GetActorForwardVector) 2e+02)) "TraceTypeQuery1" false 0 "None"))
  (for _array_element _outhits
    (bind _asbp_home_door (Utilities|Casting|CastToBP_HomeDoor (.HitActor (Collision|BreakHitResult _array_element))))
    (Variables|AIStateSwitch|SetisDoorLocked (Variables|/Game/GameplaySystems/Doors/HomeDoor/BP_HomeDoor.BP_HomeDoor_C|GetDoorLocked _asbp_home_door))
    (Variables|AIStateSwitch|SetCanSeeDoor? true)))

(event Custom|CheckForHome
  ;[1 1 1] Check for player at home(Need to optimise)
  (if (not (Variables|Init|GetIsInactive))
    (if (Variables|/Game/FirstPersonBP/Blueprints/FirstPersonCharacter.FirstPersonCharacter_C|GetIsAtHome? (Variables|Init|GetPlayerCharacter))
      (if (and (not (Variables|AIStateSwitch|GetCanSeeDoor?)) (not (Variables|AIStateSwitch|GetIsAtPlayerBase)))
        (if (not (Variables|AIStateSwitch|GetAISwitchTarget))
          (bind _closestdooractor1 (CallFunction|FindClosestDoor))
          (Variables|AIStateSwitch|SetClosest%20Door%20Actor _closestdooractor1)
          (Variables|AIStateSwitch|SetTargetLocation (Transformation|GetWorldLocation (Variables|/Game/GameplaySystems/Doors/HomeDoor/BP_HomeDoor.BP_HomeDoor_C|GetEntityLookSpot (Variables|AIStateSwitch|GetClosest%20Door%20Actor))))
          (Variables|AIStateSwitch|SetAISwitchTarget true)
          (CallFunction|HideActor))
        (else
          (Utilities|FlowControl|Sequence
            (:then_0
              (CallFunction|ShowActor))
            (:then_1
              (if (not (Variables|AIStateSwitch|GetisDoorLocked))
                (Variables|AIStateSwitch|SetAISwitchTarget false))))))
      (else
        (Variables|AIStateSwitch|SetAISwitchTarget false)))))

(event EventBeginPlay
  ;[1 1 1] Init
  (bind _asfirst_person_character (Utilities|Casting|CastToFirstPersonCharacter (Game|GetPlayerCharacter 0)))
  (Variables|Init|SetPlayerCharacter _asfirst_person_character)
  (bind _returnvalue (Utilities|Time|SetTimerbyEvent (delegate Custom|Check%20for%20Door) 0.1 true))
  (Variables|Init|SetTH_DoorCheck _returnvalue)
  ;[1 1 1] Check for player at home(Need to optimise)
  (bind _returnvalue_2 (Utilities|Time|SetTimerbyEvent (delegate Custom|CheckForHome) 0.2 true))
  (Variables|Init|SetTH_HomeCheck _returnvalue_2))

(event Collision|EventActorBeginOverlap
  (params (OtherActor :type Actor%20Object%20Reference)))

(event EventTick
  (params (DeltaSeconds :type Float%20%28single-precision%29))
  (Utilities|IsActive
    (:is%20Active
      (CallFunction|MovetoLocation (select (Variables|AIStateSwitch|GetAISwitchTarget) (Variables|AIStateSwitch|GetTargetLocation) (Transformation|GetActorLocation (Variables|Init|GetPlayerCharacter))) DeltaSeconds)
      (CallFunction|HandlePlayerDistance DeltaSeconds))))

(fn ConstructionScript)

(fn MovetoLocation
  (params (Location :type Vector) (DeltaSeconds :type Float%20%28double-precision%29))
  (Transformation|AddActorWorldOffset (* (Math|Vector|GetForwardVector (Math|Rotator|FindLookatRotation (Transformation|GetActorLocation) Location)) (* (Variables|init|GetCharacterSpeed) DeltaSeconds))))

(fn HandlePlayerDistance
  (params (DeltaSeconds :type Float%20%28double-precision%29))
  (bind _playercharacter (Variables|Init|GetPlayerCharacter))
  (bind _output_get (Variables|NearPlayer|SetPlayerDistance (Transformation|GetDistanceTo (Variables|Init|GetPlayerCharacter) self)))
  (if (< _output_get 3e+02)
    (Default|UpdateGlitchMaterialParam _playercharacter 0.51952 -0.04 0.696)
    (Default|UpdateGlitchPostProcessBlendable _playercharacter 1.0)
    (Default|DecreaseHealth (Variables|/Game/FirstPersonBP/Blueprints/FirstPersonCharacter.FirstPersonCharacter_C|GetBPC_PlayerStats (Variables|Init|GetPlayerCharacter)) (* DeltaSeconds 0.2) self)
    (else
      (Default|UpdateGlitchMaterialParam _playercharacter 0.0 0.0 0.0)
      (Default|UpdateGlitchPostProcessBlendable _playercharacter 0.0))))

(fn SetInactive
  (Variables|Init|SetIsInactive true)
  (Rendering|SetVisibility (Variables|Default|GetPS_Entity) false false)
  (Transformation|SetActorLocation "0.000000,0.000000,-2000.000000" false false))

(fn SetActive
  (Transformation|SetActorLocation (CallFunction|GetRandomSpawnLocation) false true)
  (Variables|Init|SetIsInactive false)
  (Rendering|SetVisibility (Variables|Default|GetPS_Entity) true false))

(fn FindClosestDoor
  (bind _outactors (Actor|GetAllActorsOfClass "/Game/GameplaySystems/Doors/HomeDoor/BP_HomeDoor.BP_HomeDoor_C"))
  (for (_array_element _array_index) _outactors
    (if (== _array_index 0)
      (LocalVariables|SetClosestDoorDistance (Transformation|GetDistanceTo _array_element))
      (LocalVariables|SetClosestDoorActor _array_element)
      (elif (< (Transformation|GetDistanceTo _array_element) (LocalVariables|GetClosestDoorDistance))
        (LocalVariables|SetClosestDoorDistance (Transformation|GetDistanceTo _array_element))
        (LocalVariables|SetClosestDoorActor _array_element))))
  (return (LocalVariables|GetClosestDoorActor)))

(fn HideActor
  (Rendering|SetVisibility (Variables|Default|GetPS_Entity) false false))

(fn ShowActor
  (Rendering|SetVisibility (Variables|Default|GetPS_Entity) true false))

(fn GetRandomSpawnLocation
  (bind _returnvalue (Math|Random|RandomFloatinRange 0.0 3.6e+02))
  (bind _returnvalue_2 (Math|Random|RandomFloatinRange 5e+03 1e+04))
  (bind _playercharacter (Variables|Init|GetPlayerCharacter))
  (bind _returnvalue_3 (Transformation|GetActorLocation _playercharacter))
  (return (Math|Vector|MakeVector (+ (.x _returnvalue_3) (* (Math|Trig|Cos(Degrees) _returnvalue) _returnvalue_2)) (+ (.y _returnvalue_3) (* (Math|Trig|Sin(Degrees) _returnvalue) _returnvalue_2)) (.z _returnvalue_3))))