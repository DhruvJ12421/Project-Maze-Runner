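; BP_Laser is a trap beam that damages the first-person player over time, either always active or switched on when the player's capsule enters its Box.
; While active, Tick multi-traces forward up to Range, draining health through BPCPlayerStats on player hits.
; Hit distances, or full Range on no hit, drive the beam mesh's Z scale, updated only on change.
; The construction script tints the beam through a dynamic material instance.
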(event OnComponentBeginOverlap(Box)
  (params (OverlappedComponent :type Primitive%20Component%20Object%20Reference) (OtherActor :type Actor%20Object%20Reference) (OtherComp :type Primitive%20Component%20Object%20Reference) (OtherBodyIndex :type Integer) (bFromSweep :type Boolean) (SweepResult :type Hit%20Result%20Structure%20%28by%20ref%29))
  (bind _asfirst_person_character (Utilities|Casting|CastToFirstPersonCharacter OtherActor))
  (if (== (Variables|/Script/Engine.Character|GetCapsuleComponent _asfirst_person_character) OtherComp)
    (Rendering|SetVisibility (Variables|Default|GetSM_Laser) true false)
    (Variables|Default|SetIsActive true)))

(event EventBeginPlay
  (if (Variables|Default|GetUsesBoxActivation?)
    (Rendering|SetVisibility (Variables|Default|GetSM_Laser) false false)
    (Variables|Default|SetIsActive false)
    (else
      (Variables|Default|SetIsActive true))))

(event Collision|EventActorBeginOverlap
  (params (OtherActor :type Actor%20Object%20Reference)))

(event EventTick
  (params (DeltaSeconds :type Float%20%28single-precision%29))
  (bind _returnvalue (Transformation|GetActorLocation))
  (Variables|Default|SetDelta%20Seconds DeltaSeconds)
  (if (Variables|Default|GetIsActive)
    (bind (_outhits _returnvalue_2) (Collision|MultiLineTraceByChannel _returnvalue (+ _returnvalue (* (Transformation|GetActorForwardVector) (Variables|Default|GetRange))) "TraceTypeQuery3" false 0 "ForOneFrame"))
    (if _returnvalue_2
      (for _array_element _outhits
        (Utilities|FlowControl|Sequence
          (:then_0
            (CallFunction|UpdateLength (.Distance (Collision|BreakHitResult _array_element))))
          (:then_1
            (bind _asfirst_person_character (Utilities|Casting|CastToFirstPersonCharacter (.HitActor (Collision|BreakHitResult _array_element))))
            (Default|DecreaseHealth (Variables|/Game/FirstPersonBP/Blueprints/FirstPersonCharacter.FirstPersonCharacter_C|GetBPC_PlayerStats _asfirst_person_character) (* (Variables|Default|GetDelta%20Seconds) (Variables|Default|GetDamage)) self))))
      (else
        (CallFunction|UpdateLength (Variables|Default|GetRange))))))

(fn ConstructionScript
  (bind _returnvalue (Rendering|Material|CreateDynamicMaterialInstance "/Game/GameplaySystems/Traps/Laser/Materials/MI_Laser.MI_Laser" "None" "None" :!class /Script/Engine.KismetMaterialLibrary))
  (Variables|Default|SetMaterial%20Instance _returnvalue)
  (Rendering|Material|SetMaterial (Variables|Default|GetSM_Laser) 0 (Variables|Default|GetMaterial%20Instance))
  (CallFunction|ChangeLaserColor (Variables|Default|GetColorOverride)))

(fn ChangeLaserColor
  (params (Value :type Linear%20Color%20Structure))
  (Rendering|Material|SetVectorParameterValue (Variables|Default|GetMaterial%20Instance) "Color" Value :!class /Script/Engine.MaterialInstanceDynamic))

(fn UpdateLength
  (params (Length :type Float%20%28double-precision%29))
  (if (not (Math|Float|NearlyEqual(Float) Length (Variables|Default|GetPreviousLength) 1e-06))
    (bind _output_get (Variables|Default|SetPreviousLength Length))
    (Transformation|SetWorldScale3D (Variables|Default|GetSM_Laser) (Math|Vector|MakeVector 0.1 0.1 (/ _output_get 1e+02)))))