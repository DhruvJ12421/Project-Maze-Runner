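; Player stats component that manages normalized health, regeneration and death for the first-person character.
; A looping timer slowly restores health while regeneration is allowed.
; Damage clamps health and restarts a delay timer that blocks regeneration, or at zero shows the owner's death screen, enables the cursor and pauses the game.
; Tick prints current health for debugging.
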(event Custom|RegenHealth
  (if (Variables|Default|GetCanRegen?)
    (Variables|Default|SetHealth (Math|Float|Clamp(Float) (+ (Variables|Default|GetHealth) 0.01)))))

(event Custom|DecreaseHealth
  (params (Amount :type Float%20%28double-precision%29) (DamagingActor :type Actor%20Object%20Reference))
  (bind _returnvalue (Game|GetPlayerController 0))
  (bind _ownercharacter (Variables|Default|GetOwnerCharacter))
  (bind _wdg_deathscreen (Variables|/Game/FirstPersonBP/Blueprints/FirstPersonCharacter.FirstPersonCharacter_C|GetWDG_DeathScreen _ownercharacter))
  (bind _output_get (Variables|Default|SetHealth (Math|Float|Clamp(Float) (- (Variables|Default|GetHealth) Amount))))
  (if (> _output_get 0.0)
    (Variables|Default|SetCanRegen? false)
    (if (Utilities|Time|IsValidTimerHandle (Variables|Default|GetTH_Regen))
      (Utilities|Time|ClearandInvalidateTimerbyHandle (Variables|Default|GetTH_Regen)))
    (bind _returnvalue_2 (Utilities|Time|SetTimerbyEvent (delegate Custom|CanRegenEvent) 1e+01))
    (Variables|Default|SetTH_Regen _returnvalue_2)
    (else
      ;[1 1 1] Player Death
      (if (not (UserInterface|Viewport|IsinViewport _wdg_deathscreen))
        (UserInterface|Viewport|AddtoViewport _wdg_deathscreen 0)
        (Input|SetInputModeGameandUI _returnvalue _wdg_deathscreen "DoNotLock" true false)
        (Variables|/Script/Engine.PlayerController|SetbShowMouseCursor _returnvalue true)
        (Game|SetGamePaused true)))))

(event Custom|CanRegenEvent
  (Variables|Default|SetCanRegen? true))

(event EventBeginPlay
  (bind _asfirst_person_character (Utilities|Casting|CastToFirstPersonCharacter (Game|GetPlayerCharacter 0)))
  (Variables|Default|SetOwnerCharacter _asfirst_person_character)
  (Utilities|Time|SetTimerbyEvent (delegate Custom|RegenHealth) 0.1 true))

(event EventTick
  (params (DeltaSeconds :type Float%20%28single-precision%29))
  (Utilities|FlowControl|Sequence
    (:then_0
      (Development|PrintString (Utilities|String|Append "Health : " (Utilities|String|ToString(Float) (Variables|Default|GetHealth))) true true "(R=0.000000,G=0.660000,B=1.000000,A=1.000000)" 0.0))))