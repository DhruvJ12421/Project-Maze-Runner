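; BP_Terminal is an interactable terminal NPC that pauses the game and shows a scripted chat in a WDG_Terminal widget.
; Interacting adds the IMC_Terminal input context and posts a greeting; closing the widget restores gameplay.
; IA_NextMessage steps through MessageList, auto-advancing into player messages, whose predefined text is fed to the widget on IA_Type.
; Typing-finished callbacks check each message's callback event name, though no cases are wired.
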(event Custom|StoppedUsingTerminal
  ;[1 1 1] end chatting with terminal
  (Variables|Default|SetUsingTerminal? false)
  (Widget|RemovefromParent (Variables|Default|GetWDG_Terminal))
  (Input|SetInputModeGameOnly (Game|GetPlayerController 0) false)
  (Game|SetGamePaused false)
  (Variables|/Script/Engine.PlayerController|SetbShowMouseCursor (Game|GetPlayerController 0) false)
  (Input|RemoveMappingContext (PlayerController|LocalPlayerSubsystems|GetEnhancedInputLocalPlayerSubsystem (Game|GetPlayerController 0)) "/Game/GameplaySystems/TerminalNPC/IMC_Terminal.IMC_Terminal" "(bIgnoreAllPressedKeysUntilRelease=True,bForceImmediately=False,bNotifyUserSettings=False)"))

(event Custom|First%20Terminal%20Message
  ;[1 1 1] First Terminal Message
  (Default|UpdateText (Variables|Default|GetWDG_Terminal) "HI" false))

(event Custom|UserFinishedTyping
  (Variables|Default|SetUserTyping? false)
  (CallFunction|CheckforEvents))

(event Custom|TerminalFinishedTyping
  (CallFunction|CheckforEvents))

(event Custom|CheckForEvents
  (bind _currentmessageindex (Variables|Default|GetCurrentMessageIndex))
  (bind _returnvalue (+ _currentmessageindex 1))
  ;[1 1 1] Callback Events
  (Utilities|FlowControl|Sequence
    (:then_0
      (switch name (.CallBackEventName (Utilities|Struct|BreakST_TerminalMessage (Utilities|Array|Get(acopy) (Variables|Default|GetMessageList) _currentmessageindex)))))
    (:then_1
      (if (Utilities|Array|IsValidIndex (Variables|Default|GetMessageList) _returnvalue)
        (if (Utilities|Enum|Equal(Enum) (.Type (Utilities|Struct|BreakST_TerminalMessage (Utilities|Array|Get(acopy) (Variables|Default|GetMessageList) _returnvalue))) "NewEnumerator1")
          (CallFunction|AutoNext))))))

(event Custom|AutoNext
  (bind _currentmessageindex (Variables|Default|GetCurrentMessageIndex))
  (bind _messagelist (Variables|Default|GetMessageList))
  (bind _currentmessageindex_2 (Variables|Default|GetCurrentMessageIndex))
  (bind _output (Utilities|Array|Get(acopy) _messagelist _currentmessageindex_2))
  (bind _returnvalue (+ _currentmessageindex 1))
  (bind (_message _type) (Utilities|Struct|BreakST_TerminalMessage _output))
  ;[1 1 1] Next Message
  (Utilities|CanProceed
    (:true
      (bind _result (Math|Integer|IncrementInt _currentmessageindex_2)
        (:%20%20
          (if (Utilities|Array|IsValidIndex (Variables|Default|GetMessageList) _result)
            (switch Utilities|FlowControl|Switch|SwitchonE_MessageType _type
              (:NewEnumerator0
                (if (Utilities|Array|IsValidIndex (Variables|Default|GetMessageList) _returnvalue)
                  (Default|UpdateText (Variables|Default|GetWDG_Terminal) _message (Utilities|Select :Index (.Type (Utilities|Struct|BreakST_TerminalMessage (Utilities|Array|Get(acopy) (Variables|Default|GetMessageList) _returnvalue))) :NewEnumerator0 false :NewEnumerator1 true))
                  (else
                    (Default|UpdateText (Variables|Default|GetWDG_Terminal) _message false))))
              (:NewEnumerator1
                (Variables|Default|SetUserTyping? true)))))))))

(event Input|EnhancedActionEvents|EnhancedInputActionIA_NextMessage
  (params (ActionValue :type Boolean) (ElapsedSeconds :type Float%20%28double-precision%29) (TriggeredSeconds :type Float%20%28double-precision%29) (InputAction :type Input%20Action%20Object%20Reference :default "/Game/GameplaySystems/TerminalNPC/IA_NextMessage.IA_NextMessage"))
  (bind _currentmessageindex (Variables|Default|GetCurrentMessageIndex))
  (bind _messagelist (Variables|Default|GetMessageList))
  (bind _currentmessageindex_2 (Variables|Default|GetCurrentMessageIndex))
  (bind _output (Utilities|Array|Get(acopy) _messagelist _currentmessageindex_2))
  (bind _returnvalue (+ _currentmessageindex 1))
  (bind (_message _type) (Utilities|Struct|BreakST_TerminalMessage _output))
  ;[1 1 1] Next Message
  (Utilities|CanProceed
    (:true
      (bind _result (Math|Integer|IncrementInt _currentmessageindex_2)
        (:%20%20
          (if (Utilities|Array|IsValidIndex (Variables|Default|GetMessageList) _result)
            (switch Utilities|FlowControl|Switch|SwitchonE_MessageType _type
              (:NewEnumerator0
                (if (Utilities|Array|IsValidIndex (Variables|Default|GetMessageList) _returnvalue)
                  (Default|UpdateText (Variables|Default|GetWDG_Terminal) _message (Utilities|Select :Index (.Type (Utilities|Struct|BreakST_TerminalMessage (Utilities|Array|Get(acopy) (Variables|Default|GetMessageList) _returnvalue))) :NewEnumerator0 false :NewEnumerator1 true))
                  (else
                    (Default|UpdateText (Variables|Default|GetWDG_Terminal) _message false))))
              (:NewEnumerator1
                (Variables|Default|SetUserTyping? true)))))))))

(event Input|EnhancedActionEvents|EnhancedInputActionIA_Type
  (params (ActionValue :type Boolean) (ElapsedSeconds :type Float%20%28double-precision%29) (TriggeredSeconds :type Float%20%28double-precision%29) (InputAction :type Input%20Action%20Object%20Reference :default "/Game/GameplaySystems/TerminalNPC/IA_Type.IA_Type"))
  (bind _messagelist (Variables|Default|GetMessageList))
  (bind _currentmessageindex (Variables|Default|GetCurrentMessageIndex))
  (bind _output (Utilities|Array|Get(acopy) _messagelist _currentmessageindex))
  (if (Variables|Default|GetUserTyping?)
    (switch Utilities|FlowControl|Switch|SwitchonE_MessageType (.type _output)
      (:NewEnumerator1
        (Default|PlayerUpdateText (Variables|Default|GetWDG_Terminal) (.message _output))))))

(event EventBeginPlay
  ;[1 1 1] Init
  (bind _returnvalue (UserInterface|CreateWidget "/Game/GameplaySystems/TerminalNPC/WDG_Terminal.WDG_Terminal_C"))
  (Variables|Default|SetWDG_Terminal _returnvalue)
  (EventDispatchers|BindEventtoStoppedUsingTerminal (Variables|Default|GetWDG_Terminal) (delegate Custom|StoppedUsingTerminal))
  (EventDispatchers|BindEventtoPlayerFinishedTyping (Variables|Default|GetWDG_Terminal) (delegate Custom|UserFinishedTyping))
  (EventDispatchers|BindEventtoTerminalFinishedTyping (Variables|Default|GetWDG_Terminal) (delegate Custom|TerminalFinishedTyping)))

(event EventOnInteract
  (params (InteractingActor :type First%20Person%20Character%20Object%20Reference) (InteractingComponent :type Primitive%20Component%20Object%20Reference))
  (bind _returnvalue (Game|GetPlayerController 0))
  (|CallParentFunction InteractingActor InteractingComponent)
  (Utilities|UsingTerminal
    (:false
      ;[1 1 1] Start Using Terminal
      (Utilities|FlowControl|Sequence
        (:then_0
          (UserInterface|Viewport|AddtoViewport (Variables|Default|GetWDG_Terminal) 0)
          (Input|SetInputModeGameandUI (Game|GetPlayerController 0) (Variables|Default|GetWDG_Terminal) "DoNotLock" true false)
          (Game|SetGamePaused true)
          (Variables|Default|SetUsingTerminal? true)
          (Variables|/Script/Engine.PlayerController|SetbShowMouseCursor (Game|GetPlayerController 0) true)
          (Input|EnableInput _returnvalue)
          (Input|AddMappingContext (PlayerController|LocalPlayerSubsystems|GetEnhancedInputLocalPlayerSubsystem _returnvalue) "/Game/GameplaySystems/TerminalNPC/IMC_Terminal.IMC_Terminal" 1 "(bIgnoreAllPressedKeysUntilRelease=True,bForceImmediately=False,bNotifyUserSettings=False)")
          (CallFunction|FirstTerminalMessage))))))

(fn ConstructionScript)