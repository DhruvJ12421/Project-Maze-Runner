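; AC_Scanner is a component that detects interactable actors around its owner and reports them to the player HUD.
; On BeginPlay it caches BP_PlayerHUD and starts a looping timer that repeatedly runs a multi-sphere trace on the Visibility channel at the owner's location.
; Hits implementing BPI_Interactables rebuild the list, and each addition pushes it with UsingScanner to the HUD's scanner widgets, so empty scans send no update.
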(event Custom|LookForInteractables
  (bind _returnvalue (Components|GetOwner))
  (bind _returnvalue_2 (Transformation|GetActorLocation _returnvalue))
  ;[1 1 1] Scan for interactables
  (Utilities|Array|Clear (Variables|Default|GetInteractables))
  (bind _outhits (Collision|MultiSphereTraceByChannel _returnvalue_2 _returnvalue_2 (Variables|Default|GetScannerRadius) "TraceTypeQuery1" false 0 "None"))
  (for _array_element _outhits
    (if (Utilities|DoesObjectImplementInterface (.HitActor (Collision|BreakHitResult _array_element)) "/Game/GameplaySystems/Interactables/BPI_Interactables.BPI_Interactables_C")
      (Utilities|Array|Add (Variables|Default|GetInteractables) (.HitActor (Collision|BreakHitResult _array_element)))
      (Default|UpdateScannerWidgets (Variables|Default|GetHUD) (Variables|Default|GetUsingScanner?) (Variables|Default|GetInteractables)))))

(event EventBeginPlay
  (bind _asbp_player_hud (Utilities|Casting|CastToBP_PlayerHUD (HUD|GetHUD (Game|GetPlayerController 0))))
  (Variables|Default|SetHUD _asbp_player_hud)
  (bind _returnvalue (Utilities|Time|SetTimerbyEvent (delegate Custom|LookForInteractables) 0.1 true))
  (Variables|Default|SetTH_Scan _returnvalue))