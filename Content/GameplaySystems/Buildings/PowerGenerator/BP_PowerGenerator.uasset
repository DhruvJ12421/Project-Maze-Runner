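; Power generator building, a child of a crafting building, that spends player items to temporarily add power units to its home area.
; Loading ingredients requires a valid home area with spare generation capacity and no active run, then deducts the item cost from the player's inventory.
; Power is added immediately and removed after a Delay, with the craft menu showing the generating state.
; An empty CraftItems override deliberately suppresses parent crafting.
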(event EventBeginPlay
  (|CallParentFunction)
  (Variables|Default|SetDefaultInfoText (Variables|Default|GetInfo)))

(event Collision|EventActorBeginOverlap
  (params (OtherActor :type Actor%20Object%20Reference)))

(event EventTick
  (params (DeltaSeconds :type Float%20%28single-precision%29)))

(event EventUpdateMenuData
  (bind _wdg_craftmenu (Variables|Default|GetWDG_CraftMenu))
  (Default|UpdateLeftPannel _wdg_craftmenu (Variables|Default|GetItemCost))
  (Rendering|Components|TextRender|SetText (Variables|/Game/GameplaySystems/Buildings/widgets/WDG_CraftMenu.WDG_CraftMenu_C|GetTXT_MiddlePannelHeading _wdg_craftmenu) "Unit Generated")
  (Rendering|Components|TextRender|SetText (Variables|/Game/GameplaySystems/Buildings/widgets/WDG_CraftMenu.WDG_CraftMenu_C|GetTXT_CraftedItem _wdg_craftmenu) (Utilities|Text|ToText(String) (Utilities|String|Append (Utilities|String|ToString(Integer) (Variables|Default|GetPowerUnitsGenerated)) " Units Generated")))
  (Rendering|Components|TextRender|SetText (Variables|/Game/GameplaySystems/Buildings/widgets/WDG_CraftMenu.WDG_CraftMenu_C|GetTXT_CI_Description (Variables|Default|GetWDG_CraftMenu)) (Utilities|Text|ToText(String) (Utilities|String|Append "Power Generated For " (Utilities|String|ToString(Float) (Variables|Default|GetGeneratingTime)) "s")))
  (Default|PowerGeneratorWidget (Variables|Default|GetWDG_CraftMenu))
  (Default|UpdatePlayerInventory (Variables|Default|GetWDG_CraftMenu)))

(event EventPlayerLoadIngredients
  ;[1 1 1] Power Generation and player interaction
  (Utilities|IsinHomeArea?
    (:True
      (Variables|Default|SetInfo "Generating Power")
      (if (and (not (Variables|Default|GetIsGeneratingPower?)) (Default|CanGenerateMorePower? (Variables|Default|GetHome%20Area)))
        (bind _returnvalue (Class|ACInventorySystem|DecreaseItems (Variables|/Game/FirstPersonBP/Blueprints/FirstPersonCharacter.FirstPersonCharacter_C|GetAC_InventorySystem (Variables|Default|GetPlayerCharacter)) (Variables|Default|GetItemCost)))
        (if _returnvalue
          (Default|IncreaseAvailablePowerUnits (Variables|Default|GetHome%20Area) (Variables|Default|GetPowerUnitsGenerated))
          (Variables|Default|SetIsGeneratingPower? true)
          (CallFunction|UpdateText) ; Player inventory text
          (Default|Generating (Variables|Default|GetWDG_CraftMenu))
          (Utilities|FlowControl|Delay (Variables|Default|GetGeneratingTime))
          (Variables|Default|SetIsGeneratingPower? false)
          (Default|DecreaseAvailablePowerUnits (Variables|Default|GetHome%20Area) (Variables|Default|GetPowerUnitsGenerated))
          (Default|StopGenerating (Variables|Default|GetWDG_CraftMenu)))))
    (:False
      (Variables|Default|SetInfo (Variables|Default|GetDefaultInfoText)))))

(event EventCraftItems
  ;[1 1 1] Power Generation and player interaction
)

(fn ConstructionScript)

(fn UpdateText
  (bind _playercharacter (Variables|Default|GetPlayerCharacter))
  (bind _wdg_inventory (Variables|/Game/FirstPersonBP/Blueprints/FirstPersonCharacter.FirstPersonCharacter_C|GetWDG_Inventory _playercharacter))
  (Utilities|IsValid _wdg_inventory
    (:Is%20Valid
      (Default|UpdateText _wdg_inventory))))