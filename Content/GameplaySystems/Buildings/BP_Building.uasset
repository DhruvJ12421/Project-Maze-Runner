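; Base building that the player interacts with to turn inventory items into a crafted item, with crafting skipped for power generators.
; The craft menu loads ingredients into a counted input queue and collects from an output queue into the inventory.
; Looping timers move queued items to output while powered, claim or release HomeArea power as input changes, and refresh proximity widgets.
; The HomeArea is found by sphere trace, and relocation events toggle visibility and collision.
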(event Custom|CheckNearPlayer
  ;[1 1 1] Near Player widget update
  (Rendering|SetVisibility (Variables|Default|GetBuildingWidget) (Variables|Default|GetNearPlayer) false)
  (CallFunction|UpdateInputInfo))

(event Custom|FindHomeArea
  (bind _returnvalue (Transformation|GetActorLocation))
  ;[1 1 1] FindHomeArea
  (bind _outhits (Collision|MultiSphereTraceByChannel _returnvalue _returnvalue 5e+02 "TraceTypeQuery1" false 0 "None"))
  (bind _array_element (Utilities|Array|ForEachLoopwithBreak _outhits :!label _label)
    (:LoopBody
      (bind _ashome_area (Utilities|Casting|CastToHomeArea (.HitActor (Collision|BreakHitResult _array_element))))
      (bind _output_get (Variables|Default|SetHome%20Area _ashome_area))
      (Default|AddtoBuildingList _output_get self)
      (goto _label Break))))

(event Custom|CraftClicked
  (CallFunction|PlayerLoadIngredients)
  (CallFunction|UpdateMenuData))

(event Custom|CollectClicked
  (CallFunction|PlayerCollectItems)
  (CallFunction|UpdateMenuData))

(event Custom|UpdateMenuData
  (bind _inputqueuelimit (Variables|Default|GetInputQueueLimit))
  ;[1 0.2531 0.2531] MenuData
  (Default|UpdateLeftPannel (Variables|Default|GetWDG_CraftMenu) (Variables|Default|GetItemCost))
  (Default|UpdateCraftedItemData (Variables|Default|GetWDG_CraftMenu) (not (Variables|Default|GetIsPowerGenerator?)) (Variables|Default|GetCraftedItem) _inputqueuelimit (- _inputqueuelimit (Variables|Default|GetInputQueueCount)))
  (Default|UpdateinQueueData (Variables|Default|GetWDG_CraftMenu) (Variables|Default|GetInputQueueCount) (Variables|Default|GetOutputQueueCount) (Math|Float|SelectFloat (/ (Math|Float|Round (Class|KismetSystemLibrary|GetTimerElapsedTimeHandle (Variables|Default|GetTH_Craft))) (Variables|Default|GetCrafting%20Time)) 0.0 (and (> (Variables|Default|GetInputQueueCount) 0) (Variables|Default|GetHasPower?))))
  (Default|UpdatePlayerInventory (Variables|Default|GetWDG_CraftMenu)))

(event Custom|CraftItems
  (if (CallFunction|HasIngredients?)
    (CallFunction|PopInputQueue)
    (CallFunction|PushOutputQueue)
    (CallFunction|CraftAnimations)
    (CallFunction|UpdateMenuData)))

(event Custom|PlayerLoadIngredients
  (Utilities|IsInputQueueFull?
    (:true
      (Variables|Init|SetInfo "All Slots Full"))
    (:false
      (bind _returnvalue (Class|ACInventorySystem|DecreaseItems (Variables|/Game/FirstPersonBP/Blueprints/FirstPersonCharacter.FirstPersonCharacter_C|GetAC_InventorySystem (Variables|Default|GetPlayerCharacter)) (Variables|Default|GetItemCost)))
      (if _returnvalue
        (CallFunction|PushInputQueue)
        (Utilities|UpdateText)))))

(event Custom|PlayerCollect%20Items
  (Utilities|IsNotaPowerGenerator
    (:true
      (Utilities|IsOutputQueueEmpty?
        (:false
          (CallFunction|PopOutputQueue)
          (CallFunction|AddItemtoPlayerInventory)
          (Utilities|UpdateText))))))

(event Custom|ProcessItems
  ;[1 1 1] Craft items
  (Utilities|IsNotaPowerGenerator
    (:true
      (if (Variables|Default|GetHasPower?)
        (CallFunction|CraftItems)))))

(event Custom|CraftAnimations
  (Rendering|SetVisibility (Variables|Default|GetOutputCube) true false))

(event Custom|Update%20PowerConsumption
  ;[1 1 1] Update Power
  (Utilities|IsNotaPowerGenerator
    (:true
      (if (not (Variables|/Game/GameplaySystems/Doors/HomeDoor/HomeArea.HomeArea_C|GetisSelfUpdatingPower? (Variables|Default|GetHome%20Area)))
        (CallFunction|PowerIndication)
        (if (Variables|Default|GetHasPower?)
          (if (not (CallFunction|HasIngredients?))
            (Default|StopPowerUnitConsumption (Variables|Default|GetHome%20Area) (Variables|Default|GetPowerCost))
            (Variables|Default|SetHasPower? false))
          (elif (CallFunction|HasIngredients?)
            (bind _return_value (Default|ConsumePowerUnits (Variables|Default|GetHome%20Area) (Variables|Default|GetPowerCost)))
            (Variables|Default|SetHasPower? _return_value)))))))

(event Custom|RemoveCraftMenu
  ;[1 0.3115 0.3115] Comment
  (CallFunction|RemoveCraftingMenuWidget))

(event Custom|CraftButtonClicked
  (CallFunction|PlayerLoadIngredients))

(event EventBeginPlay
  (|CallParentFunction)
  (bind _aswdg_building (Utilities|Casting|CastToWDG_Building (UserInterface|GetWidget (Variables|Default|GetBuildingWidget))))
  (Variables|init|SetWDG_Building _aswdg_building)
  (CallFunction|FindHomeArea)
  ;[1 1 1] Near Player widget update
  (bind _returnvalue (Utilities|Time|SetTimerbyEvent (delegate Custom|CheckNearPlayer) 0.1 true))
  (Variables|init|SetTH_NearPlayer _returnvalue)
  (bind _asfirst_person_character (Utilities|Casting|CastToFirstPersonCharacter (Game|GetPlayerCharacter 0)))
  (Variables|Default|SetPlayerCharacter _asfirst_person_character)
  (CallFunction|InitInputWidget)
  (CallFunction|UpdateInputInfo)
  (bind _returnvalue_2 (Utilities|Time|SetTimerbyEvent (delegate Custom|ProcessItems) (Variables|Default|GetCrafting%20Time) true))
  (Variables|Default|SetTH_Craft _returnvalue_2)
  (bind _returnvalue_3 (Utilities|Time|SetTimerbyEvent (delegate Custom|Update%20PowerConsumption) 1.0 true))
  (Variables|Default|SetTH_UpdatePower _returnvalue_3)
  (Utilities|Time|SetTimerbyEvent (EventDispatchers|CreateEvent :!event Custom|UpdateMenuData) 1.0 true)
  ;[1 0.3115 0.3115] Comment
  (bind _returnvalue_4 (UserInterface|CreateWidget "/Game/GameplaySystems/Buildings/widgets/WDG_CraftMenu.WDG_CraftMenu_C"))
  (Variables|Default|SetWDG_CraftMenu _returnvalue_4)
  (EventDispatchers|BindEventtoEDClose _returnvalue_4 (delegate Custom|RemoveCraftMenu))
  (EventDispatchers|BindEventtoEDCraft (Variables|Default|GetWDG_CraftMenu) (delegate Custom|CraftClicked))
  (EventDispatchers|BindEventtoEDCollect (Variables|Default|GetWDG_CraftMenu) (delegate Custom|CollectClicked))
  (CallFunction|UpdateMenuData)
  (Default|UpdateBuildingName (Variables|Default|GetWDG_CraftMenu) (Variables|Default|GetBuilding%20Name)))

(event EventHideActorforRelocation
  ;[1 1 1] Relocation
  (Rendering|SetActorHiddenInGame true)
  (for _array_element (Actor|GetComponentsByClass self "/Script/Engine.StaticMeshComponent")
    (bind _asstatic_mesh_component (Utilities|Casting|CastToStaticMeshComponent _array_element))
    (Collision|SetCollisionEnabled _asstatic_mesh_component "NoCollision")))

(event EventOnInteract
  (params (InteractingActor :type First%20Person%20Character%20Object%20Reference) (InteractingComponent :type Primitive%20Component%20Object%20Reference))
  (|CallParentFunction InteractingActor InteractingComponent)
  (Utilities|FlowControl|Sequence
    (:then_1
      (CallFunction|AddCraftingMenuWidget))))

(event EventShowActorAfterRelocation
  ;[1 1 1] Relocation
  (Rendering|SetActorHiddenInGame false)
  (for _array_element (Actor|GetComponentsByClass self "/Script/Engine.StaticMeshComponent")
    (bind _asstatic_mesh_component (Utilities|Casting|CastToStaticMeshComponent _array_element))
    (Collision|SetCollisionEnabled _asstatic_mesh_component "QueryAndPhysics")))

(event EventTick
  (params (DeltaSeconds :type Float%20%28single-precision%29))
  (Utilities|IsNotaPowerGenerator
    (:true
      (Development|PrintString (Utilities|String|Append "input queue : " (Utilities|String|ToString(Integer) (Variables|Default|GetInputQueueCount)) " 
" "Output Queue : " (Utilities|String|ToString(Integer) (Variables|Default|GetOutputQueueCount))) true true "(R=0.000000,G=0.660000,B=1.000000,A=1.000000)" 0.0))))

(fn ConstructionScript)

(fn InitInputWidget
  (bind _wdg_building (Variables|init|GetWDG_Building))
  (Variables|/Script/UMG.TextBlock|SetText (Variables|/Game/GameplaySystems/Buildings/widgets/WDG_Building.WDG_Building_C|GetTXT_Heading _wdg_building) (Variables|Init|GetHeading))
  (Variables|/Script/UMG.TextBlock|SetText (Variables|/Game/GameplaySystems/Buildings/widgets/WDG_Building.WDG_Building_C|GetTXT_Info _wdg_building) (Utilities|Text|ToText(String) (Variables|Init|GetInfo))))

(fn GetInputMaterialInfo
  (bind _playercharacter (Variables|Default|GetPlayerCharacter))
  (bind _ac_inventorysystem (Variables|/Game/FirstPersonBP/Blueprints/FirstPersonCharacter.FirstPersonCharacter_C|GetAC_InventorySystem _playercharacter))
  (for (_array_element _array_index) (Variables|Default|GetItemCost)
    (if (== _array_index 0)
      (LocalVariables|SetRequiredString (Utilities|String|Append (Utilities|String|ToString(Name) (.ItemName (Utilities|Struct|BreakItems (Utilities|Array|Get(acopy) (Utilities|Select :Index (.Type (Utilities|Struct|BreakDecreaseItem _array_element)) :NONE 0 :Consumables (Variables|/Script/ParkourPrototype.AC_InventorySystem|GetConsumables _ac_inventorysystem) :Parts (Variables|/Script/ParkourPrototype.AC_InventorySystem|GetParts _ac_inventorysystem) :Materials (Variables|/Script/ParkourPrototype.AC_InventorySystem|GetMaterials _ac_inventorysystem) :Tools (Variables|/Script/ParkourPrototype.AC_InventorySystem|GetTools _ac_inventorysystem)) (.index (Utilities|Struct|BreakDecreaseItem _array_element)))))) " : " (Utilities|String|ToString(Integer) (.Amount (Utilities|Struct|BreakDecreaseItem _array_element)))))
      (else
        (LocalVariables|SetRequiredString (Utilities|String|Append (LocalVariables|GetRequiredString) " 
" (Utilities|String|Append (Utilities|String|ToString(Name) (.ItemName (Utilities|Struct|BreakItems (Utilities|Array|Get(acopy) (Utilities|Select :Index (.Type (Utilities|Struct|BreakDecreaseItem _array_element)) :NONE 0 :Consumables (Variables|/Script/ParkourPrototype.AC_InventorySystem|GetConsumables _ac_inventorysystem) :Parts (Variables|/Script/ParkourPrototype.AC_InventorySystem|GetParts _ac_inventorysystem) :Materials (Variables|/Script/ParkourPrototype.AC_InventorySystem|GetMaterials _ac_inventorysystem) :Tools (Variables|/Script/ParkourPrototype.AC_InventorySystem|GetTools _ac_inventorysystem)) (.index (Utilities|Struct|BreakDecreaseItem _array_element)))))) " : " (Utilities|String|ToString(Integer) (.Amount (Utilities|Struct|BreakDecreaseItem _array_element)))))))))
  (return (LocalVariables|GetRequiredString)))

(fn UpdateInputInfo
  (Utilities|IsInputQueueFull?
    (:true
      (Variables|/Script/UMG.TextBlock|SetText (Variables|/Game/GameplaySystems/Buildings/widgets/WDG_Building.WDG_Building_C|GetTXT_Info (Variables|init|GetWDG_Building)) "All slots Full"))
    (:false
      (Variables|/Script/UMG.TextBlock|SetText (Variables|/Game/GameplaySystems/Buildings/widgets/WDG_Building.WDG_Building_C|GetTXT_Info (Variables|init|GetWDG_Building)) (Utilities|Text|ToText(String) (Utilities|String|Append (Variables|Init|GetInfo) " 
" (CallFunction|GetInputMaterialInfo))))
      (Class|ACInventorySystem|IsMissingItems (Variables|/Game/FirstPersonBP/Blueprints/FirstPersonCharacter.FirstPersonCharacter_C|GetAC_InventorySystem (Variables|Default|GetPlayerCharacter)) (Variables|Default|GetItemCost)))))

(fn HasIngredients?
  (return (> (Variables|Default|GetInputQueueCount) 0)))

(fn PushInputQueue
  (Variables|Default|SetInputQueueCount (Math|Integer|Clamp(Integer) (+ (Variables|Default|GetInputQueueCount) 1) 0 (Variables|Default|GetInputQueueLimit))))

(fn PopInputQueue
  (Variables|Default|SetInputQueueCount (Math|Integer|Clamp(Integer) (- (Variables|Default|GetInputQueueCount) 1) 0 (Variables|Default|GetInputQueueLimit))))

(fn PushOutputQueue
  (Variables|Default|SetOutputQueueCount (Math|Integer|Clamp(Integer) (+ (Variables|Default|GetOutputQueueCount) 1) 0 (Variables|Default|GetOutputQueueLimit))))

(fn PopOutputQueue
  (Variables|Default|SetOutputQueueCount (Math|Integer|Clamp(Integer) (- (Variables|Default|GetOutputQueueCount) 1) 0 (Variables|Default|GetOutputQueueLimit))))

(fn AddItemtoPlayerInventory
  (bind _crafteditem (Variables|Default|GetCraftedItem))
  (bind _playercharacter (Variables|Default|GetPlayerCharacter))
  (bind (_type _index _amount) (Utilities|Struct|BreakDecreaseItem _crafteditem))
  (bind _ac_inventorysystem (Variables|/Game/FirstPersonBP/Blueprints/FirstPersonCharacter.FirstPersonCharacter_C|GetAC_InventorySystem _playercharacter))
  (bind _consumables (Variables|/Script/ParkourPrototype.AC_InventorySystem|GetConsumables _ac_inventorysystem))
  (bind _materials (Variables|/Script/ParkourPrototype.AC_InventorySystem|GetMaterials _ac_inventorysystem))
  (bind _parts (Variables|/Script/ParkourPrototype.AC_InventorySystem|GetParts _ac_inventorysystem))
  (bind _tools (Variables|/Script/ParkourPrototype.AC_InventorySystem|GetTools _ac_inventorysystem))
  (bind _returnvalue (Utilities|Select :Index _type :NONE 0 :Consumables _consumables :Parts _parts :Materials _materials :Tools _tools))
  (bind _output (Utilities|Array|Get(acopy) _returnvalue _index))
  (bind _structout (Utilities|Struct|SetmembersinItems _output (+ (Utilities|Struct|BreakItems _output) _amount)))
  (|SetBy-RefVar _output _structout)
  (Utilities|UpdateText))

(fn PowerIndication
  (bind _home_area (Variables|Default|GetHome%20Area))
  (if (Variables|Default|GetNearPlayer)
    (if (>= (- (Variables|/Game/GameplaySystems/Doors/HomeDoor/HomeArea.HomeArea_C|GetAvailablePowerUnits _home_area) (Variables|/Game/GameplaySystems/Doors/HomeDoor/HomeArea.HomeArea_C|GetPowerUnitsConsumed _home_area)) (Variables|Default|GetPowerCost))
      (Rendering|SetVisibility (Variables|Default|GetPowerWidget) false false :!label _label)
      (Default|UpdatePowerStatus (Variables|Default|GetWDG_CraftMenu) true (Variables|Default|GetPowerCost))
      (else
        (Rendering|SetVisibility (Variables|Default|GetPowerWidget) true false)
        (Default|UpdatePowerStatus (Variables|Default|GetWDG_CraftMenu) false (Variables|Default|GetPowerCost))))
    (else
      (goto _label))))

(fn AddCraftingMenuWidget
  (bind _returnvalue (Game|GetPlayerController 0))
  (Utilities|IsValid (Variables|Default|GetWDG_CraftMenu)
    (:Is%20Valid
      (UserInterface|Viewport|AddtoViewport (Variables|Default|GetWDG_CraftMenu) 1)
      (Input|SetInputModeGameandUI _returnvalue (Variables|Default|GetWDG_CraftMenu) "DoNotLock" true false)
      (Variables|/Script/Engine.PlayerController|SetbShowMouseCursor _returnvalue true)
      (Input|RemoveMappingContext (PlayerController|LocalPlayerSubsystems|GetEnhancedInputLocalPlayerSubsystem (Game|GetPlayerController 0)) "/Game/GameplaySystems/InputSystem/MovementInputs/IMC_BasicMovement.IMC_BasicMovement" "(bIgnoreAllPressedKeysUntilRelease=True,bForceImmediately=False,bNotifyUserSettings=False)"))))

(fn RemoveCraftingMenuWidget
  (bind _returnvalue (Game|GetPlayerController 0))
  (Utilities|IsValid (Variables|Default|GetWDG_CraftMenu)
    (:Is%20Valid
      (Widget|RemovefromParent (Variables|Default|GetWDG_CraftMenu))
      (Input|SetInputModeGameOnly _returnvalue false)
      (Variables|/Script/Engine.PlayerController|SetbShowMouseCursor _returnvalue false)
      (Input|AddMappingContext (PlayerController|LocalPlayerSubsystems|GetEnhancedInputLocalPlayerSubsystem (Game|GetPlayerController 0)) "/Game/GameplaySystems/InputSystem/MovementInputs/IMC_BasicMovement.IMC_BasicMovement" 0 "(bIgnoreAllPressedKeysUntilRelease=True,bForceImmediately=False,bNotifyUserSettings=False)"))))