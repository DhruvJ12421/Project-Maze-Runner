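; Building actor for base building that serves as a placement hologram and then as the placed structure.
; On BeginPlay it async loads its data asset and then that asset's static mesh, destroying itself if the soft reference is invalid.
; CanPlaceBuild box traces slightly shrunken mesh bounds on Visibility, setting validity and a blue or red hologram material.
; PlaceBuilding restores the default material and enables query and physics collision.
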(event EventBeginPlay
  (if (Utilities|IsValidSoftObjectReference (Variables|Default|GetDataAssetUsed))
    (bind _object (Utilities|AsyncLoadAsset (Variables|Default|GetDataAssetUsed))
      (:Completed
        (bind _asda_blueprint (Utilities|Casting|CastToDA_Blueprint _object))
        (bind _object_2 (Utilities|AsyncLoadAsset (Variables|/Game/GameplaySystems/Buildings/BaseBuilding/DataAssets/DA_Blueprint.DA_Blueprint_C|GetStaticMesh _asda_blueprint))
          (:Completed
            (bind _asstatic_mesh (Utilities|Casting|CastToStaticMesh _object_2))
            (Components|StaticMesh|SetStaticMesh (Variables|Default|GetStaticMesh) _asstatic_mesh)))))
    (else
      (Actor|DestroyActor))))

(fn ConstructionScript)

(fn CanPlaceBuild
  (bind _staticmesh (Variables|Default|GetStaticMesh))
  (bind _origin (Collision|GetComponentBounds _staticmesh))
  (bind _returnvalue (Collision|BoxTraceByChannel _origin _origin (* (- (.Max (Components|StaticMesh|GetLocalBounds _staticmesh)) (Math|Transform|InverseTransformLocation (Transformation|GetActorTransform) _origin)) 0.88) (Transformation|GetActorRotation) "TraceTypeQuery1" false 0 "ForOneFrame"))
  (Variables|Default|SetIsValidPlacement? (not _returnvalue))
  (Rendering|Material|SetMaterial (Variables|Default|GetStaticMesh) 0 (select (Variables|Default|GetIsValidPlacement?) "/Game/GameplaySystems/Buildings/BaseBuilding/Materials/MI_Hologram2_Blue.MI_Hologram2_Blue" "/Game/GameplaySystems/Buildings/BaseBuilding/Materials/MI_Hologram2_Red.MI_Hologram2_Red")))

(fn PlaceBuilding
  (Rendering|Material|SetMaterial (Variables|Default|GetStaticMesh) 0 "/Engine/EngineMaterials/DefaultMaterial.DefaultMaterial")
  (Collision|SetCollisionEnabled (Variables|Default|GetStaticMesh) "QueryAndPhysics"))