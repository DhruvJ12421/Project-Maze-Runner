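; Actor component that runs the player's base-building mode on a home grid, with a pausing menu for choosing among collected building blueprints by type.
; A selection spawns a preview BP_SpawnedBuilding that follows a camera line trace each tick, checking placement validity until confirmed.
; Previews snap to tile centers and grid-aligned quarter turns; holding the grid input allows free placement with finer rotation, and holding freeze stops movement.
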(event Custom|CloseBuildMenu
  (bind _returnvalue (Game|GetPlayerController 0))
  (Widget|RemovefromParent (Variables|Default|GetBuildMenu))
  (Input|SetInputModeGameOnly _returnvalue false)
  (Variables|/Script/Engine.PlayerController|SetbShowMouseCursor _returnvalue false)
  (Game|SetGamePaused false))

(event Custom|SelectedBuilding
  (params (SelectedBuilding :type ST%20Building%20Blueprint%20Structure))
  (bind _output_get (Variables|Default|SetSelected%20Building SelectedBuilding))
  (Utilities|Map|Add (Variables|init|GetBuildingMap) 0 (.ClassReference (Utilities|Struct|BreakST_BuildingBlueprint _output_get)))
  (BuildTool|SpawnNewBuild (.Value (Utilities|Map|Find (Variables|init|GetBuildingMap) (Math|Float|Round 0.0)))))

(event Input|EnhancedActionEvents|EnhancedInputActionIA_BuildSelect
  (params (ActionValue :type Float%20%28double-precision%29) (ElapsedSeconds :type Float%20%28double-precision%29) (TriggeredSeconds :type Float%20%28double-precision%29) (InputAction :type Input%20Action%20Object%20Reference :default "/Game/GameplaySystems/Buildings/BaseBuilding/Inputs/IA_BuildSelect.IA_BuildSelect"))
  (:Started
    (Utilities|IsinBuildMode
      (:true
        (BuildTool|SpawnNewBuild (.Value (Utilities|Map|Find (Variables|init|GetBuildingMap) (- (Math|Float|Round ActionValue) 1))))))))

(event Input|EnhancedActionEvents|EnhancedInputActionIA_Grid
  (params (ActionValue :type Boolean) (ElapsedSeconds :type Float%20%28double-precision%29) (TriggeredSeconds :type Float%20%28double-precision%29) (InputAction :type Input%20Action%20Object%20Reference :default "/Game/GameplaySystems/Buildings/BaseBuilding/Inputs/IA_Grid.IA_Grid"))
  (:Started
    (Utilities|IsinBuildMode
      (:true
        _)
      (:false
        _))
    (Variables|Init|SetIsUsingGrid? false))
  (:Canceled
    (Utilities|IsinBuildMode :!label _label
      (:true
        (Variables|Init|SetIsUsingGrid? true)
        (bind _buildingreference (Variables|Init|GetBuildingReference)
          (:then
            (Transformation|SetActorRotation _buildingreference (BuildTool|GetSpawnRotation)))
          (:else)))))
  (:Completed
    (goto _label)))

(event Input|EnhancedActionEvents|EnhancedInputActionIA_Rotate
  (params (ActionValue :type Float%20%28double-precision%29) (ElapsedSeconds :type Float%20%28double-precision%29) (TriggeredSeconds :type Float%20%28double-precision%29) (InputAction :type Input%20Action%20Object%20Reference :default "/Game/GameplaySystems/Buildings/BaseBuilding/Inputs/IA_Rotate.IA_Rotate"))
  (bind _isusinggrid_ (Variables|Init|GetIsUsingGrid?))
  (bind _returnvalue (Math|Float|SelectFloat 9e+01 1e+01 _isusinggrid_))
  (:Started
    (Utilities|IsinBuildMode
      (:true
        (bind _buildingreference (Variables|Init|GetBuildingReference)
          (:then
            (Class|Actor|AddActorWorldRotation _buildingreference (Math|Rotator|MakeRotator 0.0 0.0 (Math|Float|MapRangeClamped ActionValue -1.0 1.0 (* _returnvalue -1.0) _returnvalue))))
          (:else))))))

(event Input|EnhancedActionEvents|EnhancedInputActionIA_Confirm
  (params (ActionValue :type Boolean) (ElapsedSeconds :type Float%20%28double-precision%29) (TriggeredSeconds :type Float%20%28double-precision%29) (InputAction :type Input%20Action%20Object%20Reference :default "/Game/GameplaySystems/Buildings/BaseBuilding/Inputs/IA_Confirm.IA_Confirm"))
  (:Started
    (Utilities|IsinBuildMode
      (:true
        (bind _buildingreference (Variables|Init|GetBuildingReference)
          (:then
            (if (Variables|/Game/GameplaySystems/Buildings/BaseBuilding/Blueprints/BP_SpawnedBuilding.BP_SpawnedBuilding_C|GetIsValidPlacement? _buildingreference)
              (Default|PlaceBuilding (Variables|Init|GetBuildingReference))
              (Variables|Init|SetBuildingReference 0)
              (Default|SetTileVisibility (Variables|Init|GetHomeGrid) false)))
          (:else))))))

(event Input|EnhancedActionEvents|EnhancedInputActionIA_BuildMode
  (params (ActionValue :type Boolean) (ElapsedSeconds :type Float%20%28double-precision%29) (TriggeredSeconds :type Float%20%28double-precision%29) (InputAction :type Input%20Action%20Object%20Reference :default "/Game/GameplaySystems/Buildings/BaseBuilding/Inputs/IA_BuildMode.IA_BuildMode"))
  (:Started
    (bind _homegrid (Variables|Init|GetHomeGrid)
      (:then
        (Default|ToggleGrid _homegrid)
        (BuildTool|ToggleBuildMode))
      (:else))))

(event Input|EnhancedActionEvents|EnhancedInputActionIA_BuildMenu
  (params (ActionValue :type Boolean) (ElapsedSeconds :type Float%20%28double-precision%29) (TriggeredSeconds :type Float%20%28double-precision%29) (InputAction :type Input%20Action%20Object%20Reference :default "/Game/GameplaySystems/Buildings/BaseBuilding/Inputs/IA_BuildMenu.IA_BuildMenu"))
  (bind _returnvalue (Game|GetPlayerController 0))
  (bind _returnvalue_2 (Game|GetPlayerController 0))
  (Utilities|IsinBuildMode
    (:true
      (if (not (UserInterface|Viewport|IsinViewport (Variables|Default|GetBuildMenu)))
        (UserInterface|Viewport|AddtoViewport (Variables|Default|GetBuildMenu) 1)
        (Input|SetInputModeGameandUI _returnvalue_2 (Variables|Default|GetBuildMenu) "DoNotLock" true false)
        (Variables|/Script/Engine.PlayerController|SetbShowMouseCursor _returnvalue_2 true)
        (Game|SetGamePaused true)
        (Default|UpdateBlueprints (Variables|Default|GetBuildMenu) (Variables|BuildData|GetGeneratorBlueprints) (Variables|BuildData|GetRefinerBlueprints) (Variables|BuildData|GetAmmunitionConverter) (Variables|BuildData|GetSkillManifestor))
        (else
          (Widget|RemovefromParent (Variables|Default|GetBuildMenu))
          (Input|SetInputModeGameOnly _returnvalue false)
          (Variables|/Script/Engine.PlayerController|SetbShowMouseCursor _returnvalue false)
          (Game|SetGamePaused false))))))

(event Input|EnhancedActionEvents|EnhancedInputActionIA_Freeze
  (params (ActionValue :type Boolean) (ElapsedSeconds :type Float%20%28double-precision%29) (TriggeredSeconds :type Float%20%28double-precision%29) (InputAction :type Input%20Action%20Object%20Reference :default "/Game/GameplaySystems/Buildings/BaseBuilding/Inputs/IA_Freeze.IA_Freeze"))
  ;[1 1 1] Freeze
  (:Started
    (Utilities|IsinBuildMode
      (:true
        (Variables|Default|SetisFrozen? true))))
  (:Canceled
    (Variables|Default|SetisFrozen? false :!label _label))
  (:Completed
    (goto _label)))

(event EventBeginPlay
  (Input|AddMappingContext (PlayerController|LocalPlayerSubsystems|GetEnhancedInputLocalPlayerSubsystem (Game|GetPlayerController 0)) "/Game/GameplaySystems/Buildings/BaseBuilding/Inputs/IMC_Building.IMC_Building" 0 "(bIgnoreAllPressedKeysUntilRelease=True,bForceImmediately=False,bNotifyUserSettings=False)")
  (bind _returnvalue (UserInterface|CreateWidget "/Game/GameplaySystems/Buildings/GeneralSystems/WDG_BuildMenu.WDG_BuildMenu_C"))
  (bind _output_get (Variables|Default|SetBuildMenu _returnvalue))
  (EventDispatchers|BindEventtoCloseBuildMenu _output_get (EventDispatchers|CreateEvent :!event Custom|CloseBuildMenu))
  (EventDispatchers|BindEventtoUpdateSelectedBuild (Variables|Default|GetBuildMenu) (EventDispatchers|CreateEvent :!event Custom|SelectedBuilding)))

(event EventTick
  (params (DeltaSeconds :type Float%20%28single-precision%29))
  (Utilities|IsinBuildMode
    (:true
      (if (not (Variables|Default|GetisFrozen?))
        (BuildTool|UpdateBuildLocation)))))

(fn SpawnNewBuild
  (params (InputPin :type DA%20Blueprint%20Soft%20Object%20Reference))
  (bind _buildingreference (Variables|Init|GetBuildingReference)
    (:then
      (Actor|DestroyActor _buildingreference))
    (:else
      _))
  (bind _outhit (Utilities|LineTracebyChannelFWD))
  (bind _returnvalue (Game|SpawnActorfromClass "/Game/GameplaySystems/Buildings/BaseBuilding/Blueprints/BP_SpawnedBuilding.BP_SpawnedBuilding_C" (Math|Transform|MakeTransform (.ImpactPoint (Collision|BreakHitResult _outhit)) (BuildTool|GetSpawnRotation) "1.000000,1.000000,1.000000") "Undefined" "MultiplyWithRoot" 0 InputPin (.AsPawn (Utilities|Casting|CastToPawn (Components|GetOwner)))))
  (Variables|Init|SetBuildingReference _returnvalue))

(fn UpdateBuildLocation
  (Variables|Init|GetBuildingReference
    (:then
      (Utilities|FlowControl|Sequence
        (:then_0
          (bind _outhit (Utilities|LineTracebyChannelFWD))
          (bind _homegrid (Variables|Init|GetHomeGrid)
            (:then
              (Default|SetSelectedTileViaLocation _homegrid (.ImpactPoint (Collision|BreakHitResult _outhit)))
              (bind (_isvalid_ _centerlocation) (Default|LocationtoGridCenter _homegrid (.ImpactPoint (Collision|BreakHitResult _outhit)))))
            (:else
              _))
          (Transformation|SetActorLocation (Variables|Init|GetBuildingReference) (Math|Vector|SelectVector _centerlocation (.ImpactPoint (Collision|BreakHitResult _outhit)) (and _isvalid_ (Variables|Init|GetIsUsingGrid?))) false false))
        (:then_1
          (Default|CanPlaceBuild (Variables|Init|GetBuildingReference)))))
    (:else)))

(fn GetSpawnRotation
  (bind _homegrid (Variables|Init|GetHomeGrid))
  (bind _returnvalue (Transformation|GetActorRotation _homegrid))
  (bind _yaw (Math|Rotator|BreakRotator _returnvalue))
  (return (Math|Rotator|MakeRotator 0.0 0.0 (select (Utilities|IsValid (Variables|Init|GetHomeGrid)) (+ (* (Math|Float|Round (/ (- (.Yaw (Math|Rotator|BreakRotator (Transformation|GetActorRotation (Components|GetOwner)))) _yaw) 9e+01)) 90) _yaw) (.Yaw (Math|Rotator|BreakRotator (Transformation|GetActorRotation (Components|GetOwner))))))))

(fn ToggleBuildMode
  (if (Variables|Init|GetBuildMode?)
    (Variables|Init|SetBuildMode? false)
    (Variables|Init|SetIsUsingGrid? false)
    (bind _buildingreference (Variables|Init|GetBuildingReference)
      (:then
        (Actor|DestroyActor _buildingreference))
      (:else))
    (else
      (Variables|Init|GetHomeGrid
        (:then
          (Variables|Init|SetBuildMode? true)
          (Variables|Init|SetIsUsingGrid? true))
        (:else)))))

(fn EndBuildMode
  (Variables|Init|SetBuildMode? false)
  (Variables|Init|SetIsUsingGrid? false)
  (Default|SetGridVisibility (Variables|Init|GetHomeGrid) false)
  (bind _buildingreference (Variables|Init|GetBuildingReference)
    (:then
      (Actor|DestroyActor _buildingreference))
    (:else)))

(fn AddNewBlueprint
  (params (Blueprint :type ST%20Building%20Blueprint%20Structure))
  (switch Utilities|FlowControl|Switch|SwitchonE_BuildingType (.BuildingType (Utilities|Struct|BreakST_BuildingBlueprint Blueprint))
    (:NewEnumerator0
      (Utilities|Array|Add (Variables|BuildData|GetGeneratorBlueprints) Blueprint))
    (:NewEnumerator1
      (Utilities|Array|Add (Variables|BuildData|GetRefinerBlueprints) Blueprint))
    (:NewEnumerator2
      (Utilities|Array|Add (Variables|BuildData|GetSkillManifestor) Blueprint))
    (:NewEnumerator3
      (Utilities|Array|Add (Variables|BuildData|GetAmmunitionConverter) Blueprint))))