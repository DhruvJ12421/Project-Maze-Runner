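; Base-building grid actor that draws a tile grid with a selection highlight and converts between world locations and tiles.
; The construction script builds both as procedural meshes of flat quads from CreateLine, each with its own dynamic instance of M_Grid.
; Helper functions validate tiles, return corners or snapped centers, and move the highlight to a chosen tile.
; Both meshes start hidden on BeginPlay, with functions to show or toggle them.
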(event EventBeginPlay
  (Rendering|SetVisibility (Variables|Default|GetSelectionProceduralMesh) false false)
  (Rendering|SetVisibility (Variables|Default|GetLinesProceduralMesh) false false))

(fn ConstructionScript
  (bind _tilesize (Variables|Constants|GetTileSize))
  (bind _returnvalue (/ _tilesize 2.0))
  ;[1 1 1] Init Material Instance
  (bind _materialinstance (Private|CreateMaterialInstance (Variables|Constants|GetLineColor) (Variables|Constants|GetLineOpacity) (Variables|Constants|GetLineOpaqueDistance) (Variables|Constants|GetLineFadeDistance) (Variables|Constants|GetLineEmissivity)))
  (LocalVariables|SetLinesMaterialInstance _materialinstance)
  (bind _materialinstance_2 (Private|CreateMaterialInstance (Variables|Constants|GetSelectionColor) (Variables|Constants|GetSelectionOpacity) (* (Math|Integer|Max(Integer) (Variables|Constants|GetNumColumns) (Variables|Constants|GetNumRows)) (Variables|Constants|GetTileSize)) 2e+02 (Variables|Constants|GetSelectionEmissivity)))
  (LocalVariables|SetSelectionMaterialInstance _materialinstance_2)
  (Utilities|FlowControl|Sequence
    (:then_0
      ;[1 1 1] Create Horizontal line geometry
      (for _index (range 0 (Variables|Constants|GetNumRows))
        (LocalVariables|SetLineStart (* _index (Variables|Constants|GetTileSize)))
        (LocalVariables|SetLineEnd (Private|GridWidth))
        (Private|CreateLine (Math|Vector|MakeVector (LocalVariables|GetLineStart) 0.0 0.0) (Math|Vector|MakeVector (LocalVariables|GetLineStart) (LocalVariables|GetLineEnd) 0.0) (Variables|Constants|GetLineThickness) (LocalVariables|GetLineVertices) (LocalVariables|GetLineTriangles))))
    (:then_1
      ;[1 1 1] Create Vertical line geometry
      (for _index_2 (range 0 (Variables|Constants|GetNumColumns))
        (LocalVariables|SetLineStart (* _index_2 (Variables|Constants|GetTileSize)))
        (LocalVariables|SetLineEnd (Private|GridHeight))
        (Private|CreateLine (Math|Vector|MakeVector 0.0 (LocalVariables|GetLineStart) 0.0) (Math|Vector|MakeVector (LocalVariables|GetLineEnd) (LocalVariables|GetLineStart) 0.0) (Variables|Constants|GetLineThickness) (LocalVariables|GetLineVertices) (LocalVariables|GetLineTriangles))))
    (:then_2
      ;[1 1 1] Creating procedural mesh for the lines
      (Class|ProceduralMeshComponent|CreateMeshSectionLinearColor (Variables|Default|GetLinesProceduralMesh) 0 (LocalVariables|GetLineVertices) (LocalVariables|GetLineTriangles) 0 0 0 0 0 0 0 false false)
      (Rendering|Material|SetMaterial (Variables|Default|GetLinesProceduralMesh) 0 (LocalVariables|GetLinesMaterialInstance)))
    (:then_3
      ;[1 1 1] Create selection geomety and creating a procedural mesh for it
      (Private|CreateLine (Math|Vector|MakeVector 0.0 _returnvalue 0.0) (Math|Vector|MakeVector (Variables|Constants|GetTileSize) _returnvalue 0.0) (Variables|Constants|GetTileSize) (LocalVariables|GetSelectionVertices) (LocalVariables|GetSelectionTriangles))
      (Class|ProceduralMeshComponent|CreateMeshSectionLinearColor (Variables|Default|GetSelectionProceduralMesh) 0 (LocalVariables|GetSelectionVertices) (LocalVariables|GetSelectionTriangles) 0 0 0 0 0 0 0 false false)
      (Rendering|Material|SetMaterial (Variables|Default|GetSelectionProceduralMesh) 0 (LocalVariables|GetSelectionMaterialInstance)))))

(fn CreateLine
  (params (Start :type Vector) (End :type Vector) (Thickness :type Float%20%28double-precision%29) (vertices :type Array%20of%20Vectors) (Triangles :type Array%20of%20Integers))
  (bind _returnvalue (Utilities|Array|Length vertices))
  (Utilities|FlowControl|Sequence
    (:then_0
      (LocalVariables|SetHalfThickness (/ Thickness 2.0))
      (LocalVariables|SetThicknessDirection (Math|Vector|CrossProduct (Math|Vector|Normalize (- End Start)) "0.000000,0.000000,1.000000")))
    (:then_1
      (Utilities|Array|AppendArray Triangles (Utilities|Array|MakeArray (+ _returnvalue 2) (+ _returnvalue 1) (+ _returnvalue 0) (+ _returnvalue 2) (+ _returnvalue 3) (+ _returnvalue 1)))
      (Utilities|Array|AppendArray vertices (Utilities|Array|MakeArray (+ Start (* (LocalVariables|GetThicknessDirection) (LocalVariables|GetHalfThickness))) (+ End (* (LocalVariables|GetThicknessDirection) (LocalVariables|GetHalfThickness))) (- Start (* (LocalVariables|GetThicknessDirection) (LocalVariables|GetHalfThickness))) (- End (* (LocalVariables|GetThicknessDirection) (LocalVariables|GetHalfThickness))))))))

(fn GridWidth
  (return (* (Variables|Constants|GetNumColumns) (Variables|Constants|GetTileSize))))

(fn GridHeight
  (return (* (Variables|Constants|GetNumRows) (Variables|Constants|GetTileSize))))

(fn CreateMaterialInstance
  (params (Color :type Linear%20Color%20Structure) (Opacity :type Float%20%28double-precision%29) (M_OpaqueDistance :type Float%20%28double-precision%29) (M_FadeDistance :type Float%20%28double-precision%29) (M_Emissivity :type Float%20%28double-precision%29))
  (bind _returnvalue (Rendering|Material|CreateDynamicMaterialInstance "/Game/GameplaySystems/Buildings/BaseBuilding/Grid/M_Grid.M_Grid" "None" "None" :!class /Script/Engine.KismetMaterialLibrary))
  (Rendering|Material|SetVectorParameterValue _returnvalue "Color" Color :!class /Script/Engine.MaterialInstanceDynamic)
  (Rendering|Material|SetScalarParameterValue _returnvalue "Opacity" Opacity :!class /Script/Engine.MaterialInstanceDynamic)
  (Rendering|Material|SetScalarParameterValue _returnvalue "Emissivity" M_Emissivity :!class /Script/Engine.MaterialInstanceDynamic)
  (Rendering|Material|SetScalarParameterValue _returnvalue "MaxOpaqueDistance" M_OpaqueDistance :!class /Script/Engine.MaterialInstanceDynamic)
  (Rendering|Material|SetScalarParameterValue _returnvalue "FadeDistance" M_FadeDistance :!class /Script/Engine.MaterialInstanceDynamic)
  (return _returnvalue))

(fn LocationtoTile
  (params (Location :type Vector))
  (bind _returnvalue (Private|GridHeight))
  (bind _returnvalue_2 (Transformation|GetActorLocation))
  (bind _returnvalue_3 (Transformation|GetActorLocation))
  (bind _width (Private|GridWidth))
  (bind _numrows (Variables|Constants|GetNumRows))
  (bind _numcolumns (Variables|Constants|GetNumColumns))
  (bind _returnvalue_4 (- (.y Location) (.y _returnvalue_2)))
  (bind _returnvalue_5 (- (.x Location) (.x _returnvalue_3)))
  (bind _returnvalue_6 (/ _returnvalue_4 _returnvalue))
  (bind _returnvalue_7 (/ _returnvalue_5 _width))
  (bind _returnvalue_8 (* _numcolumns _returnvalue_6))
  (bind _returnvalue_9 (* _numrows _returnvalue_7))
  (bind _returnvalue_10 (Math|Float|Floor _returnvalue_8))
  (bind _returnvalue_11 (Math|Float|Floor _returnvalue_9))
  (bind _valid_ (Utilities|IsTileValid _returnvalue_11 _returnvalue_10))
  (return _returnvalue_11 _returnvalue_10 _valid_))

(fn TiletoGridLocation
  (params (Row :type Integer) (Column :type Integer) (Center? :type Boolean))
  (bind _tilesize (Variables|Constants|GetTileSize))
  (bind _returnvalue (/ _tilesize 2.0))
  (bind _returnvalue_2 (select Center? _returnvalue 0.0))
  (bind _valid_ (Utilities|IsTileValid Row Column))
  (return _valid_ (Math|Vector|MakeVector (+ (+ (* Row (Variables|Constants|GetTileSize)) (.x (Transformation|GetActorLocation))) _returnvalue_2) (+ _returnvalue_2 (+ (* Column (Variables|Constants|GetTileSize)) (.y (Transformation|GetActorLocation)))) (.z (Transformation|GetActorLocation)))))

(fn SetSelectedTile
  (params (Row :type Integer) (Column :type Integer))
  (bind _selectionproceduralmesh (Variables|Default|GetSelectionProceduralMesh))
  (bind (_isvalid _gridlocation) (Public|TiletoGridLocation Row Column false))
  (if _isvalid
    (Rendering|SetVisibility _selectionproceduralmesh true false)
    (Transformation|SetWorldLocation (Variables|Default|GetSelectionProceduralMesh) (Math|Vector|MakeVector (.X (Math|Vector|BreakVector _gridlocation)) (.Y (Math|Vector|BreakVector _gridlocation)) (.Z (Math|Vector|BreakVector _gridlocation))) false false)
    (else
      (Rendering|SetVisibility _selectionproceduralmesh false false))))

(fn ToggleGrid
  (Rendering|ToggleVisibility (Variables|Default|GetLinesProceduralMesh) false)
  (Rendering|SetVisibility (Variables|Default|GetSelectionProceduralMesh) false false))

(fn LocationtoGridCenter
  (params (Location :type Vector))
  (bind (_row _column) (Public|LocationtoTile Location))
  (bind (_isvalid _gridlocation) (Public|TiletoGridLocation _row _column true))
  (return _isvalid _gridlocation))

(fn SetSelectedTileViaLocation
  (params (Location :type Vector))
  (bind (_row _column _isvalid) (Public|LocationtoTile Location))
  (if _isvalid
    (Public|SetSelectedTile _row _column)))

(fn SetGridVisibility
  (params (NewVisibility :type Boolean))
  (Rendering|SetVisibility (Variables|Default|GetSelectionProceduralMesh) NewVisibility false)
  (Rendering|SetVisibility (Variables|Default|GetLinesProceduralMesh) NewVisibility false))

(fn SetTileVisibility
  (params (Visibility :type Boolean))
  (Rendering|SetVisibility (Variables|Default|GetSelectionProceduralMesh) Visibility false))

(fn GetGrid
  (return self))