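; BP_HomeDoor is the home's sliding door, whose lock wears down on a timer while locked and forces the door open at zero health.
; Full or partial repairs spend inventory items scaled by health restored, then relock it, with costs shown on a widget visible near the player.
; A timeline moves the door vertically, driven by interaction, Outside/Inside overlaps and a polling timer that closes it once the player leaves.
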(event OnComponentBeginOverlap(Inside)
  (params (OverlappedComponent :type Primitive%20Component%20Object%20Reference) (OtherActor :type Actor%20Object%20Reference) (OtherComp :type Primitive%20Component%20Object%20Reference) (OtherBodyIndex :type Integer) (bFromSweep :type Boolean) (SweepResult :type Hit%20Result%20Structure%20%28by%20ref%29))
  (Utilities|Casting|CastToFirstPersonCharacter OtherActor)
  (if (Variables|Default|GetWasOutside?)
    (CallFunction|CloseDoor)
    (Variables|Default|SetWasOutside? false)))

(event OnComponentBeginOverlap(Outside)
  (params (OverlappedComponent :type Primitive%20Component%20Object%20Reference) (OtherActor :type Actor%20Object%20Reference) (OtherComp :type Primitive%20Component%20Object%20Reference) (OtherBodyIndex :type Integer) (bFromSweep :type Boolean) (SweepResult :type Hit%20Result%20Structure%20%28by%20ref%29))
  (Utilities|Casting|CastToFirstPersonCharacter OtherActor)
  (CallFunction|OpenDoor)
  (Variables|Default|SetWasOutside? true))

(event Custom|Open%20Door
  ;[1 1 1] OpenDoor
  (Variables|LockStats|SetDoorLocked false)
  (Variables|Default|SetInteractMessage "")
  (bind _alpha (Timeline|OpenDoor Play)
    (:Update
      (Transformation|SetRelativeLocation (Variables|Default|GetPlaceHolderDoor) (Math|Vector|MakeVector 0.0 0.0 (Math|Float|Lerp 2.3e+02 7.3e+02 _alpha)) false true))
    (:Finished
      (if (not (Variables|LockStats|GetDoorLocked))
        (bind _returnvalue (Utilities|Time|SetTimerbyEvent (delegate Custom|PlayerCheckForLocking) 0.1 true))
        (Variables|Init|SetTH_DoorLock _returnvalue)))))

(event Custom|CloseDoor
  ;[1 1 1] OpenDoor
  (if (Variables|LockStats|GetCanLockDoor?)
    (Variables|LockStats|SetDoorLocked true)
    (Variables|Default|SetInteractMessage "Press RMB to Open Door")
    (bind _alpha (Timeline|OpenDoor Reverse)
      (:Update
        (Transformation|SetRelativeLocation (Variables|Default|GetPlaceHolderDoor) (Math|Vector|MakeVector 0.0 0.0 (Math|Float|Lerp 2.3e+02 7.3e+02 _alpha)) false true))
      (:Finished
        (if (not (Variables|LockStats|GetDoorLocked))
          (bind _returnvalue (Utilities|Time|SetTimerbyEvent (delegate Custom|PlayerCheckForLocking) 0.1 true))
          (Variables|Init|SetTH_DoorLock _returnvalue))))))

(event Custom|ReplenishDoorLockHealth
  (bind _playercharacter (Variables|init|GetPlayerCharacter))
  (bind _wdg_inventory (Variables|/Game/FirstPersonBP/Blueprints/FirstPersonCharacter.FirstPersonCharacter_C|GetWDG_Inventory _playercharacter))
  ;[1 1 1] Replenish Lock Health
  (bind _returnvalue (Class|ACInventorySystem|DecreaseItems (Variables|/Game/FirstPersonBP/Blueprints/FirstPersonCharacter.FirstPersonCharacter_C|GetAC_InventorySystem (Variables|init|GetPlayerCharacter)) (CallFunction|RequiredAmounttoRepair)))
  (if _returnvalue
    (Variables|LockStats|SetLockHealth 1.0)
    (Utilities|IsValid _wdg_inventory
      (:Is%20Valid
        (Default|UpdateText _wdg_inventory))
      (:Is%20Not%20Valid
        _))
    (CallFunction|UpdateWidget)
    (Variables|LockStats|SetCanLockDoor? true)
    (CallFunction|CloseDoor)))

(event Custom|ReplenishCompletelyBind
  ;[1 1 1] Initialization
  ;;[1 1 1] UI binding
  (CallFunction|ReplenishDoorLockHealth))

(event Custom|WDG_Display
  ;[1 1 1] Near Visibility
  (Rendering|SetVisibility (Variables|Default|GetWDG_Door) (Variables|Default|GetNearPlayer) false))

(event Custom|ReduceLockHealth
  ;[1 1 1] ReduceLockHealth
  (if (<= (Variables|LockStats|GetLockHealth) 0.0)
    (Variables|LockStats|SetDoorLocked false)
    (Variables|LockStats|SetCanLockDoor? false)
    (CallFunction|OpenDoor)
    (elif (Variables|LockStats|GetDoorLocked) ; Reduce Health Only when door is locked
      (Variables|LockStats|SetLockHealth (Math|Float|Clamp(Float) (- (Variables|LockStats|GetLockHealth) (Variables|LockStats|GetHealthDecreaseRate))))
      (CallFunction|UpdateWidget (CallFunction|RequiredAmounttoRepair)))))

(event Custom|ReplenishHealthPartially
  (params (Percent :type Float%20%28double-precision%29))
  (bind _returnvalue (Math|Float|Clamp(Float) Percent))
  (bind _playercharacter (Variables|init|GetPlayerCharacter))
  (bind _wdg_inventory (Variables|/Game/FirstPersonBP/Blueprints/FirstPersonCharacter.FirstPersonCharacter_C|GetWDG_Inventory _playercharacter))
  ;[1 1 1] Replenish Lock Health
  (bind _requireditems (CallFunction|RepairCostforXPercent _returnvalue))
  (bind _returnvalue_2 (Class|ACInventorySystem|DecreaseItems (Variables|/Game/FirstPersonBP/Blueprints/FirstPersonCharacter.FirstPersonCharacter_C|GetAC_InventorySystem (Variables|init|GetPlayerCharacter)) _requireditems))
  (if _returnvalue_2
    (Variables|LockStats|SetLockHealth (+ (Variables|LockStats|GetLockHealth) _returnvalue))
    (Utilities|IsValid _wdg_inventory
      (:Is%20Valid
        (Default|UpdateText _wdg_inventory))
      (:Is%20Not%20Valid
        _))
    (CallFunction|UpdateWidget (CallFunction|RequiredAmounttoRepair))
    (Variables|LockStats|SetCanLockDoor? true)
    (CallFunction|CloseDoor)))

(event Custom|PlayerCheckForLocking
  ;[1 1 1] OpenDoor
  (if (not (Variables|Default|GetNearPlayer))
    (CallFunction|CloseDoor)
    (Utilities|Time|ClearandInvalidateTimerbyHandle (Variables|Init|GetTH_DoorLock))))

(event Custom|ReplenishPartiallyBind
  ;[1 1 1] Initialization
  ;;[1 1 1] UI binding
  (CallFunction|ReplenishHealthPartially (Variables|/Game/GameplaySystems/Doors/HomeDoor/WDG_HomeDoor.WDG_HomeDoor_C|GetPercent (Variables|Init|GetWDGDoor))))

(event Custom|Update%20PartialRepairEvent
  ;[1 1 1] Initialization
  ;;[1 1 1] UI binding
  (CallFunction|UpdateRepairPartialCost (Variables|/Game/GameplaySystems/Doors/HomeDoor/WDG_HomeDoor.WDG_HomeDoor_C|GetPercent (Variables|Init|GetWDGDoor))))

(event EventBeginPlay
  ;[1 1 1] Initialization
  (bind _asfirst_person_character (Utilities|Casting|CastToFirstPersonCharacter (Game|GetPlayerCharacter 0)))
  (Variables|init|SetPlayerCharacter _asfirst_person_character)
  (bind _aswdg_home_door (Utilities|Casting|CastToWDG_HomeDoor (UserInterface|GetWidget (Variables|Default|GetWDG_Door))))
  (Variables|Init|SetWDGDoor _aswdg_home_door)
  (CallFunction|UpdateWidget (CallFunction|RequiredAmounttoRepair))
  (EventDispatchers|BindEventtoReplenishCompletely (Variables|Init|GetWDGDoor) (delegate Custom|ReplenishCompletelyBind))
  (EventDispatchers|BindEventtoReplenishPartially (Variables|Init|GetWDGDoor) (delegate Custom|ReplenishPartiallyBind))
  (EventDispatchers|BindEventtoUpdatePartialRepairText (Variables|Init|GetWDGDoor) (delegate Custom|Update%20PartialRepairEvent))
  ;[1 1 1] Near Visibility
  (Utilities|Time|SetTimerbyEvent (delegate Custom|WDG_Display) 0.1 true)
  ;[1 1 1] Reduce Lock health
  (bind _returnvalue (Utilities|Time|SetTimerbyEvent (delegate Custom|ReduceLockHealth) (Variables|LockStats|GetReduceTimeInterval) true))
  (Variables|Init|SetTH_ReduceHealth _returnvalue))

(event EventOnInteract
  (params (InteractingActor :type First%20Person%20Character%20Object%20Reference) (InteractingComponent :type Primitive%20Component%20Object%20Reference))
  (CallFunction|OpenDoor))

(fn ConstructionScript)

(fn RequiredAmounttoRepair
  (for _array_element (Variables|LockStats|GetLockFullRepairCost)
    (bind _output_get (LocalVariables|SetTemp%28Local%29 (Utilities|Struct|MakeDecreaseItem (.Type (Utilities|Struct|BreakDecreaseItem _array_element)) (.index (Utilities|Struct|BreakDecreaseItem _array_element)) (Math|Float|Ceil (* (.Amount (Utilities|Struct|BreakDecreaseItem _array_element)) (- 1.0 (/ (Variables|LockStats|GetLockHealth) (Variables|LockStats|GetLockMaxHealth))))))))
    (if (> (.amount (LocalVariables|GetTemp%28Local%29)) 0)
      (Utilities|Array|Add (LocalVariables|GetCostOfRepair) _output_get)))
  (return (LocalVariables|GetCostOfRepair)))

(fn MinRepairAmount
  (for _array_element (CallFunction|RequiredAmounttoRepair)
    (bind _output_get (LocalVariables|SetTemp (Utilities|Struct|MakeDecreaseItem (.Type (Utilities|Struct|BreakDecreaseItem _array_element)) (.index (Utilities|Struct|BreakDecreaseItem _array_element)) 1)))
    (Utilities|Array|Add (LocalVariables|GetMinReqItems%28local%29) _output_get))
  (return (LocalVariables|GetMinReqItems%28local%29)))

(fn UpdateWidget
  (params (RequiredAmount :type Array%20of%20Decrease%20Item%20Structures))
  (bind _playercharacter (Variables|init|GetPlayerCharacter))
  (bind _ac_inventorysystem (Variables|/Game/FirstPersonBP/Blueprints/FirstPersonCharacter.FirstPersonCharacter_C|GetAC_InventorySystem _playercharacter))
  (Utilities|FlowControl|Sequence
    (:then_0
      (bind _aswdg_home_door (Utilities|Casting|CastToWDG_HomeDoor (UserInterface|GetWidget (Variables|Default|GetWDG_Door))))
      (LocalVariables|SetWDG_Door%28Local%29 _aswdg_home_door)
      (Variables|/Game/GameplaySystems/Doors/HomeDoor/WDG_HomeDoor.WDG_HomeDoor_C|SetMaxHealth _aswdg_home_door (Variables|LockStats|GetLockMaxHealth))
      (Variables|/Game/GameplaySystems/Doors/HomeDoor/WDG_HomeDoor.WDG_HomeDoor_C|SetLockHealth _aswdg_home_door (Variables|LockStats|GetLockHealth))
      (Variables|/Game/GameplaySystems/Doors/HomeDoor/WDG_HomeDoor.WDG_HomeDoor_C|SetPercent _aswdg_home_door 0.0)
      (CallFunction|UpdateRepairPartialCost 0.0))
    (:then_1
      (Variables|/Script/UMG.TextBlock|SetText (Variables|/Game/GameplaySystems/Doors/HomeDoor/WDG_HomeDoor.WDG_HomeDoor_C|GetTXT_Items (LocalVariables|GetWDG_Door%28Local%29)) ""))
    (:then_2
      (for (_array_element _array_index) RequiredAmount
        (Variables|/Script/UMG.TextBlock|SetText (Variables|/Game/GameplaySystems/Doors/HomeDoor/WDG_HomeDoor.WDG_HomeDoor_C|GetTXT_Items (LocalVariables|GetWDG_Door%28Local%29)) (Utilities|Text|ToText(String) (select (== _array_index 0) (Utilities|String|Append (Utilities|String|ToString(Name) (.itemname (Utilities|Array|Get(acopy) (Utilities|Select :Index (.Type (Utilities|Struct|BreakDecreaseItem _array_element)) :NONE 0 :Consumables (Variables|/Script/ParkourPrototype.AC_InventorySystem|GetConsumables _ac_inventorysystem) :Parts (Variables|/Script/ParkourPrototype.AC_InventorySystem|GetParts _ac_inventorysystem) :Materials (Variables|/Script/ParkourPrototype.AC_InventorySystem|GetMaterials _ac_inventorysystem) :Tools (Variables|/Script/ParkourPrototype.AC_InventorySystem|GetTools _ac_inventorysystem)) (.index (Utilities|Struct|BreakDecreaseItem _array_element))))) " : " (Utilities|String|ToString(Integer) (.Amount (Utilities|Struct|BreakDecreaseItem _array_element)))) (Utilities|String|Append (Utilities|String|ToString(Text) (Variables|/Script/UMG.TextBlock|GetText (Variables|/Game/GameplaySystems/Doors/HomeDoor/WDG_HomeDoor.WDG_HomeDoor_C|GetTXT_Items (LocalVariables|GetWDG_Door%28Local%29)))) " 
" (Utilities|String|Append (Utilities|String|ToString(Name) (.itemname (Utilities|Array|Get(acopy) (Utilities|Select :Index (.Type (Utilities|Struct|BreakDecreaseItem _array_element)) :NONE 0 :Consumables (Variables|/Script/ParkourPrototype.AC_InventorySystem|GetConsumables _ac_inventorysystem) :Parts (Variables|/Script/ParkourPrototype.AC_InventorySystem|GetParts _ac_inventorysystem) :Materials (Variables|/Script/ParkourPrototype.AC_InventorySystem|GetMaterials _ac_inventorysystem) :Tools (Variables|/Script/ParkourPrototype.AC_InventorySystem|GetTools _ac_inventorysystem)) (.index (Utilities|Struct|BreakDecreaseItem _array_element))))) " : " (Utilities|String|ToString(Integer) (.Amount (Utilities|Struct|BreakDecreaseItem _array_element))))))))))))

(fn RepairCostforXPercent
  (params (Percentage :type Float%20%28double-precision%29))
  (if (> Percentage 0.0)
    (for _array_element (Variables|LockStats|GetLockFullRepairCost)
      (bind _output_get (LocalVariables|SetTemp%28Local%29 (Utilities|Struct|MakeDecreaseItem (.Type (Utilities|Struct|BreakDecreaseItem _array_element)) (.index (Utilities|Struct|BreakDecreaseItem _array_element)) (Math|Float|Ceil (* (.Amount (Utilities|Struct|BreakDecreaseItem _array_element)) Percentage)))))
      (Utilities|Array|Add (LocalVariables|GetRequiredItem) _output_get))
    (return (LocalVariables|GetRequiredItem))
    (else
      (return 0))))

(fn UpdateRepairPartialCost
  (params (Percent :type Float%20%28double-precision%29))
  (bind _playercharacter (Variables|init|GetPlayerCharacter))
  (bind _ac_inventorysystem (Variables|/Game/FirstPersonBP/Blueprints/FirstPersonCharacter.FirstPersonCharacter_C|GetAC_InventorySystem _playercharacter))
  (Utilities|FlowControl|Sequence
    (:then_0
      (Variables|/Script/UMG.TextBlock|SetText (Variables|/Game/GameplaySystems/Doors/HomeDoor/WDG_HomeDoor.WDG_HomeDoor_C|GetTXT_MinCost (Variables|Init|GetWDGDoor)) ""))
    (:then_1
      (bind _requireditems (CallFunction|RepairCostforXPercent (Math|Float|Clamp(Float) Percent)))
      (for (_array_element _array_index) _requireditems
        (Variables|/Script/UMG.TextBlock|SetText (Variables|/Game/GameplaySystems/Doors/HomeDoor/WDG_HomeDoor.WDG_HomeDoor_C|GetTXT_MinCost (Variables|Init|GetWDGDoor)) (Utilities|Text|ToText(String) (select (== _array_index 0) (Utilities|String|Append (Utilities|String|ToString(Name) (.itemname (Utilities|Array|Get(acopy) (Utilities|Select :Index (.Type (Utilities|Struct|BreakDecreaseItem _array_element)) :NONE 0 :Consumables (Variables|/Script/ParkourPrototype.AC_InventorySystem|GetConsumables _ac_inventorysystem) :Parts (Variables|/Script/ParkourPrototype.AC_InventorySystem|GetParts _ac_inventorysystem) :Materials (Variables|/Script/ParkourPrototype.AC_InventorySystem|GetMaterials _ac_inventorysystem) :Tools (Variables|/Script/ParkourPrototype.AC_InventorySystem|GetTools _ac_inventorysystem)) (.index (Utilities|Struct|BreakDecreaseItem _array_element))))) " : " (Utilities|String|ToString(Integer) (.Amount (Utilities|Struct|BreakDecreaseItem _array_element)))) (Utilities|String|Append (Utilities|String|ToString(Text) (Variables|/Script/UMG.TextBlock|GetText (Variables|/Game/GameplaySystems/Doors/HomeDoor/WDG_HomeDoor.WDG_HomeDoor_C|GetTXT_MinCost (Variables|Init|GetWDGDoor)))) " 
" (Utilities|String|Append (Utilities|String|ToString(Name) (.itemname (Utilities|Array|Get(acopy) (Utilities|Select :Index (.Type (Utilities|Struct|BreakDecreaseItem _array_element)) :NONE 0 :Consumables (Variables|/Script/ParkourPrototype.AC_InventorySystem|GetConsumables _ac_inventorysystem) :Parts (Variables|/Script/ParkourPrototype.AC_InventorySystem|GetParts _ac_inventorysystem) :Materials (Variables|/Script/ParkourPrototype.AC_InventorySystem|GetMaterials _ac_inventorysystem) :Tools (Variables|/Script/ParkourPrototype.AC_InventorySystem|GetTools _ac_inventorysystem)) (.index (Utilities|Struct|BreakDecreaseItem _array_element))))) " : " (Utilities|String|ToString(Integer) (.Amount (Utilities|Struct|BreakDecreaseItem _array_element))))))))))))