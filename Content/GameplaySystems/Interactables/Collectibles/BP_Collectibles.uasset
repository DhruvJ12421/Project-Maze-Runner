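; Collectible item actor that the player picks up into the inventory component on interact, or on overlapping its box while E is held.
; GetItemStruct supplies the item data for its info widget, which a looping timer shows or hides from NearPlayer.
; Pickup passes a never-reset DoOnce, then a carry-weight check, before updating count and weight.
; A successful pickup plays a shrink-and-spin timeline, then destroys the actor.
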(event OnComponentBeginOverlap(Box_0)
  (params (OverlappedComponent :type Primitive%20Component%20Object%20Reference) (OtherActor :type Actor%20Object%20Reference) (OtherComp :type Primitive%20Component%20Object%20Reference) (OtherBodyIndex :type Integer) (bFromSweep :type Boolean) (SweepResult :type Hit%20Result%20Structure%20%28by%20ref%29))
  (bind _ownercharacter (Variables|Default|GetOwnerCharacter))
  (bind _ownercharacter_2 (Variables|Default|GetOwnerCharacter))
  (bind _itemstruct (Utilities|GetItemStruct _ownercharacter_2))
  (bind _ac_inventorysystem (Variables|/Game/FirstPersonBP/Blueprints/FirstPersonCharacter.FirstPersonCharacter_C|GetAC_InventorySystem _ownercharacter_2))
  (bind _wdg_inventory (Variables|/Game/FirstPersonBP/Blueprints/FirstPersonCharacter.FirstPersonCharacter_C|GetWDG_Inventory _ownercharacter))
  (Utilities|Casting|CastToFirstPersonCharacter OtherActor)
  (if (Variables|/Game/GameplaySystems/Interactables/BPC_PlayerInteractionComponent.BPC_PlayerInteractionComponent_C|GetEKeyDown (Variables|/Game/FirstPersonBP/Blueprints/FirstPersonCharacter.FirstPersonCharacter_C|GetBPC_PlayerInteractionComponent (Variables|Default|GetOwnerCharacter)))
    (Utilities|FlowControl|DoOnce false
      (:Completed
        (if (<= (+ (.itemweight _itemstruct) (Variables|/Script/ParkourPrototype.AC_InventorySystem|GetItemCarryAmount _ac_inventorysystem)) (Variables|/Script/ParkourPrototype.AC_InventorySystem|GetMaxInventoryCapacity _ac_inventorysystem))
          (Math|Integer|IncrementInt (.count _itemstruct)
            (:%20%20
              (Variables|/Script/ParkourPrototype.AC_InventorySystem|SetItemCarryAmount (Variables|/Game/FirstPersonBP/Blueprints/FirstPersonCharacter.FirstPersonCharacter_C|GetAC_InventorySystem _ownercharacter) (+ (.itemweight _itemstruct) (Variables|/Script/ParkourPrototype.AC_InventorySystem|GetItemCarryAmount _ac_inventorysystem)))
              ;[1 0.3043 0.1542] Temporary(DEBUG)
              (Utilities|IsValid _wdg_inventory
                (:Is%20Valid
                  (Default|UpdateText _wdg_inventory))
                (:Is%20Not%20Valid
                  _))
              (Utilities|Time|ClearandInvalidateTimerbyHandle (Variables|Default|GetTHItemDisplay))
              (Variables|Default|SetOriginalScale (Transformation|GetActorScale3D))
              (bind _alphasize (Timeline|ReduceSizeAndRotate Play)
                (:Update
                  (Transformation|SetActorRelativeScale3D (Math|Vector|Lerp(Vector) "0.100000,0.100000,0.100000" (Variables|Default|GetOriginalScale) _alphasize))
                  (Transformation|AddActorLocalRotation "7.000000,7.000000,7.000000" false false))
                (:Finished
                  (Actor|DestroyActor))))))))))

(event Custom|ItemInfoDisplay
  (Rendering|SetVisibility (Variables|Default|GetWDG_ItemInfo) (Variables|Default|GetNearPlayer) false))

(event EventBeginPlay
  (Utilities|FlowControl|Sequence
    (:then_0
      (bind _returnvalue (Utilities|Time|SetTimerbyEvent (delegate Custom|ItemInfoDisplay) 0.1 true))
      (Variables|Default|SetTHItemDisplay _returnvalue))
    (:then_1
      ;[1 1 1] ItemDescription init
      (bind _asfirst_person_character (Utilities|Casting|CastToFirstPersonCharacter (Game|GetPlayerCharacter 0)))
      (bind _output_get (Variables|Default|SetOwnerCharacter _asfirst_person_character))
      (CallFunction|SetCollectibleDescription (Utilities|Text|ToText(Name) (.itemname (Utilities|GetItemStruct _output_get))) (Utilities|Text|ToText(String) (.description (Utilities|GetItemStruct _output_get))) (.itemweight (Utilities|GetItemStruct _output_get))))))

(event EventOnInteract
  (params (InteractingActor :type First%20Person%20Character%20Object%20Reference) (InteractingComponent :type Primitive%20Component%20Object%20Reference))
  (bind _ownercharacter (Variables|Default|GetOwnerCharacter))
  (bind _ownercharacter_2 (Variables|Default|GetOwnerCharacter))
  (bind _itemstruct (Utilities|GetItemStruct _ownercharacter_2))
  (bind _ac_inventorysystem (Variables|/Game/FirstPersonBP/Blueprints/FirstPersonCharacter.FirstPersonCharacter_C|GetAC_InventorySystem _ownercharacter_2))
  (bind _wdg_inventory (Variables|/Game/FirstPersonBP/Blueprints/FirstPersonCharacter.FirstPersonCharacter_C|GetWDG_Inventory _ownercharacter))
  (Utilities|FlowControl|DoOnce false
    (:Completed
      (if (<= (+ (.itemweight _itemstruct) (Variables|/Script/ParkourPrototype.AC_InventorySystem|GetItemCarryAmount _ac_inventorysystem)) (Variables|/Script/ParkourPrototype.AC_InventorySystem|GetMaxInventoryCapacity _ac_inventorysystem))
        (Math|Integer|IncrementInt (.count _itemstruct)
          (:%20%20
            (Variables|/Script/ParkourPrototype.AC_InventorySystem|SetItemCarryAmount (Variables|/Game/FirstPersonBP/Blueprints/FirstPersonCharacter.FirstPersonCharacter_C|GetAC_InventorySystem _ownercharacter) (+ (.itemweight _itemstruct) (Variables|/Script/ParkourPrototype.AC_InventorySystem|GetItemCarryAmount _ac_inventorysystem)))
            ;[1 0.3043 0.1542] Temporary(DEBUG)
            (Utilities|IsValid _wdg_inventory
              (:Is%20Valid
                (Default|UpdateText _wdg_inventory))
              (:Is%20Not%20Valid
                _))
            (Utilities|Time|ClearandInvalidateTimerbyHandle (Variables|Default|GetTHItemDisplay))
            (Variables|Default|SetOriginalScale (Transformation|GetActorScale3D))
            (bind _alphasize (Timeline|ReduceSizeAndRotate Play)
              (:Update
                (Transformation|SetActorRelativeScale3D (Math|Vector|Lerp(Vector) "0.100000,0.100000,0.100000" (Variables|Default|GetOriginalScale) _alphasize))
                (Transformation|AddActorLocalRotation "7.000000,7.000000,7.000000" false false))
              (:Finished
                (Actor|DestroyActor)))))))))

(fn ConstructionScript)

(fn SetCollectibleDescription
  (params (ItemName :type Text) (ItemDescription :type Text) (ItemWeight :type Integer))
  (bind _aswdg_collectible_message (Utilities|Casting|CastToWDG_CollectibleMessage (UserInterface|GetWidget (Variables|Default|GetWDG_ItemInfo))))
  (Variables|/Script/UMG.TextBlock|SetText (Variables|/Game/GameplaySystems/Interactables/Collectibles/WDG_CollectibleMessage.WDG_CollectibleMessage_C|GetTXT_Name _aswdg_collectible_message) ItemName)
  (Variables|/Script/UMG.TextBlock|SetText (Variables|/Game/GameplaySystems/Interactables/Collectibles/WDG_CollectibleMessage.WDG_CollectibleMessage_C|GetTXT_Description _aswdg_collectible_message) ItemDescription)
  (Variables|/Script/UMG.TextBlock|SetText (Variables|/Game/GameplaySystems/Interactables/Collectibles/WDG_CollectibleMessage.WDG_CollectibleMessage_C|GetTXT_Weight _aswdg_collectible_message) (Utilities|Text|ToText(String) (Utilities|String|Append "Item Weight : " (Utilities|String|ToString(Integer) ItemWeight)))))