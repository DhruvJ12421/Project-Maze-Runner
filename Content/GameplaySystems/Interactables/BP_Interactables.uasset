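; Interactable actor that shows its Interactable component while the player is near and exposes a scanner detection box through a getter.
; DiscoverThemselves shows the component, sets NearPlayer and, guarded by a DoOnce, starts a looping one-second timer instead of using Tick.
; Each check compares player distance against the interaction component's discovery radius; beyond it, the component hides, the timer clears, the DoOnce resets and NearPlayer turns false.
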(event EventBeginPlay)

(event Collision|EventActorBeginOverlap
  (params (OtherActor :type Actor%20Object%20Reference)))

(event EventDiscoverThemselves
  ;[1 1 1] Near Player Discovery
  (Rendering|SetVisibility (Variables|Default|GetInteractable) true false)
  (Variables|Default|SetNearPlayer true)
  (Utilities|FlowControl|DoOnce false
    (:Completed
      (bind _returnvalue (Utilities|Time|SetTimerbyEvent (delegate EventCheckforPlayer) 1.0 true))
      (Variables|Default|SetPlayerCheckEvent _returnvalue))))

(event EventCheckforPlayer
  ;[1 1 1] Near Player Discovery
  (bind _asfirst_person_character (Utilities|Casting|CastToFirstPersonCharacter (Game|GetPlayerCharacter 0)))
  (if (> (Transformation|GetDistanceTo _asfirst_person_character self) (Variables|/Game/GameplaySystems/Interactables/BPC_PlayerInteractionComponent.BPC_PlayerInteractionComponent_C|GetInteractableDiscoveryRadius (Variables|/Game/FirstPersonBP/Blueprints/FirstPersonCharacter.FirstPersonCharacter_C|GetBPC_PlayerInteractionComponent _asfirst_person_character)))
    (Rendering|SetVisibility (Variables|Default|GetInteractable) false false)
    (Utilities|FlowControl|Sequence
      (:then_0
        (Utilities|Time|ClearandInvalidateTimerbyHandle (Variables|Default|GetPlayerCheckEvent))
        (Utilities|FlowControl|DoOnce false) ; enters at Reset
      )
      (:then_1
        (Variables|Default|SetNearPlayer false)))))

(fn ConstructionScript)

(fn GetScannerDetectionBox
  (return (Variables|Default|GetScannerDetectionBox)))