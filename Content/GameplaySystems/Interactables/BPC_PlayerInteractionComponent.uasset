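; Player interaction component for the first-person character that finds nearby interactables, shows an interact prompt and forwards interact input.
; A looping timer sphere-traces around the player and sends a discover message to interface implementers in clear line of sight.
; A faster timer line-traces from the camera to cache the looked-at actor for input.
; For collectibles, the prompt turns into a red warning when inventory capacity would be exceeded.
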(event Custom|CheckForInteractables
  (bind _ownercharacter (Variables|Default|GetOwnerCharacter))
  (bind _returnvalue (Transformation|GetActorLocation _ownercharacter))
  ;[1 1 1] Sphere Trace For Interactables
  (bind _outhits (Collision|MultiSphereTraceByChannel _returnvalue _returnvalue (Variables|Default|GetInteractableDiscoveryRadius) "TraceTypeQuery1" false (Utilities|Array|MakeArray _ownercharacter) "None"))
  (for _array_element _outhits
    (if (Utilities|DoesObjectImplementInterface (.HitActor (Collision|BreakHitResult _array_element)) "/Game/GameplaySystems/Interactables/BPI_Interactables.BPI_Interactables_C")
      (if (CallFunction|IsVisibletoPlayer (.HitActor (Collision|BreakHitResult _array_element)))
        (Class|BPIInteractables|DiscoverThemselves(Message) (.HitActor (Collision|BreakHitResult _array_element)))))))

(event Custom|CheckForReachableInteractables
  (bind _ownercharacter (Variables|Default|GetOwnerCharacter))
  (bind _firstpersoncamera (Variables|/Game/FirstPersonBP/Blueprints/FirstPersonCharacter.FirstPersonCharacter_C|GetFirstPersonCamera _ownercharacter))
  (bind _returnvalue (Transformation|GetWorldLocation _firstpersoncamera))
  ;[1 1 1] LineTrace From Camera for interaction of nearby Actor
  (Utilities|FlowControl|Sequence
    (:then_0
      (bind _outhit (Collision|LineTraceByChannel _returnvalue (+ _returnvalue (* (Math|Vector|GetForwardVector _firstpersoncamera) 2e+02)) "TraceTypeQuery1" false (Utilities|Array|MakeArray (Variables|Default|GetOwnerCharacter)) "None"))
      (if (Utilities|DoesObjectImplementInterface (.HitActor (Collision|BreakHitResult _outhit)) "/Game/GameplaySystems/Interactables/BPI_Interactables.BPI_Interactables_C")
        (if (and (not (UserInterface|Viewport|IsinViewport (Variables|Default|GetInteractWidget))) (!= (.HitActor (Collision|BreakHitResult _outhit)) (Variables|Default|GetPlayerLookAtActor)))
          (bind _asbp_interactables (Utilities|Casting|CastToBP_Interactables (.HitActor (Collision|BreakHitResult _outhit)))
            (:then
              (CallFunction|CollectibleCapacityCheck (.HitActor (Collision|BreakHitResult _outhit)) (Variables|/Game/GameplaySystems/Interactables/BP_Interactables.BP_Interactables_C|GetInteractMessage _asbp_interactables)) ; changes both text and color of widget
            )
            (:CastFailed
              (Variables|/Script/UMG.TextBlock|SetText (Variables|/Game/GameplaySystems/Interactables/WDG_InteractPrompt.WDG_InteractPrompt_C|GetTXT_Interact (Variables|Default|GetInteractWidget)) (Variables|/Game/GameplaySystems/Interactables/BP_Interactables.BP_Interactables_C|GetInteractMessage _asbp_interactables))))
          (UserInterface|Viewport|AddtoViewport (Variables|Default|GetInteractWidget) 0)
          (Variables|Default|SetPlayerLookAtActor (.HitActor (Collision|BreakHitResult _outhit)))
          (Variables|Default|SetPlayerLookAtComponenet (.HitComponent (Collision|BreakHitResult _outhit))))
        (else
          (Widget|RemovefromParent (Variables|Default|GetInteractWidget))
          (Variables|Default|SetPlayerLookAtActor 0))))))

(event Input|EnhancedActionEvents|EnhancedInputActionIA_Interact
  (params (ActionValue :type Boolean) (ElapsedSeconds :type Float%20%28double-precision%29) (TriggeredSeconds :type Float%20%28double-precision%29) (InputAction :type Input%20Action%20Object%20Reference :default "/Game/GameplaySystems/InputSystem/General/IA_Interact.IA_Interact"))
  (bind _playerlookatactor (Variables|Default|GetPlayerLookAtActor))
  ;[1 1 1] Interact
  (:Started
    (Variables|Default|SetEKeyDown true)
    (Utilities|IsValid _playerlookatactor
      (:Is%20Valid
        (Class|BPIInteractables|OnInteract(Message) _playerlookatactor (Variables|Default|GetOwnerCharacter) (Variables|Default|GetPlayerLookAtComponenet)))))
  (:Completed
    (Utilities|FlowControl|Delay 0.2)
    (Variables|Default|SetEKeyDown false)))

(event EventBeginPlay
  ;[1 1 1] Setup
  (bind _returnvalue (UserInterface|CreateWidget "/Game/GameplaySystems/Interactables/WDG_InteractPrompt.WDG_InteractPrompt_C"))
  (Variables|Default|SetInteractWidget _returnvalue)
  (bind _asfirst_person_character (Utilities|Casting|CastToFirstPersonCharacter (Components|GetOwner)))
  (Variables|Default|SetOwnerCharacter _asfirst_person_character)
  (bind _returnvalue_2 (Utilities|Time|SetTimerbyEvent (delegate Custom|CheckForInteractables) 0.2 true))
  ;[1 1 1] LineTrace From Camera for interaction of nearby Actor
  (Variables|Default|SetTH_InteractableCheck _returnvalue_2)
  (Utilities|Time|SetTimerbyEvent (delegate Custom|CheckForReachableInteractables) 0.1 true))

(event Input|ActionEvents|InputActionInteract
  (params (Key :type Key%20Structure :default "None")))

(fn IsVisibletoPlayer
  (params (Actor :type Actor%20Object%20Reference))
  (bind _returnvalue (Transformation|GetActorLocation Actor))
  (bind _ownercharacter (Variables|Default|GetOwnerCharacter))
  (bind _returnvalue_2 (Transformation|GetActorLocation _ownercharacter))
  (if (<= (Math|Vector|Distance(Vector) _returnvalue_2 _returnvalue) (Variables|Default|GetInteractableDiscoveryRadius))
    (bind _outhit (Collision|LineTraceByChannel _returnvalue_2 _returnvalue "TraceTypeQuery1" false (Utilities|Array|MakeArray (Variables|Default|GetOwnerCharacter)) "None"))
    (return (== Actor (.HitActor (Collision|BreakHitResult _outhit))))
    (else
      (return false))))

(fn CollectibleCapacityCheck
  (params (HitActor :type Actor%20Object%20Reference) (OriginalMessage :type Text))
  (bind _ownercharacter (Variables|Default|GetOwnerCharacter))
  (bind _interactwidget (Variables|Default|GetInteractWidget))
  (bind _interactwidget_2 (Variables|Default|GetInteractWidget))
  (bind _txt_interact (Variables|/Game/GameplaySystems/Interactables/WDG_InteractPrompt.WDG_InteractPrompt_C|GetTXT_Interact _interactwidget))
  (bind _ac_inventorysystem (Variables|/Game/FirstPersonBP/Blueprints/FirstPersonCharacter.FirstPersonCharacter_C|GetAC_InventorySystem _ownercharacter))
  (bind _txt_interact_2 (Variables|/Game/GameplaySystems/Interactables/WDG_InteractPrompt.WDG_InteractPrompt_C|GetTXT_Interact _interactwidget_2))
  (bind _asbp_collectibles (Utilities|Casting|CastToBP_Collectibles HitActor)
    (:then
      (if (<= (+ (.itemweight (Utilities|GetItemStruct (Variables|/Game/GameplaySystems/Interactables/Collectibles/BP_Collectibles.BP_Collectibles_C|GetCollectibleType _asbp_collectibles) _asbp_collectibles)) (Variables|/Script/ParkourPrototype.AC_InventorySystem|GetItemCarryAmount _ac_inventorysystem)) (Variables|/Script/ParkourPrototype.AC_InventorySystem|GetMaxInventoryCapacity _ac_inventorysystem))
        (Variables|/Script/UMG.TextBlock|SetText _txt_interact_2 OriginalMessage :!label _label)
        (Appearance|SetColorandOpacity _txt_interact_2 (Utilities|Struct|MakeSlateColor "(R=1.000000,G=1.000000,B=1.000000,A=1.000000)" "UseColor_Specified") :!class /Script/UMG.TextBlock)
        (else
          (Variables|/Script/UMG.TextBlock|SetText _txt_interact "Not Enough Space")
          (Appearance|SetColorandOpacity _txt_interact (Utilities|Struct|MakeSlateColor "(R=0.841667,G=0.000000,B=0.017792,A=1.000000)" "UseColor_Specified") :!class /Script/UMG.TextBlock))))
    (:CastFailed
      (goto _label))))