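; Interactable generator in the ability bench system that trades inventory items for double jump cells.
; On interact, it asks the owner character's inventory component to deduct the item cost.
; If that succeeds, it adds the cell amount to the count of the first Tools slot by index, keeping its other fields, then refreshes the inventory widget text.
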(event Collision|EventActorBeginOverlap
  (params (OtherActor :type Actor%20Object%20Reference)))

(event EventTick
  (params (DeltaSeconds :type Float%20%28single-precision%29)))

(event EventOnInteract
  (params (InteractingActor :type First%20Person%20Character%20Object%20Reference))
  (bind _ownercharacter (Variables|Default|GetOwnerCharacter))
  (bind _ownercharacter_2 (Variables|Default|GetOwnerCharacter))
  (bind _ac_inventorysystem (Variables|/Game/FirstPersonBP/Blueprints/FirstPersonCharacter.FirstPersonCharacter_C|GetAC_InventorySystem _ownercharacter_2))
  (bind _ac_inventorysystem_2 (Variables|/Game/FirstPersonBP/Blueprints/FirstPersonCharacter.FirstPersonCharacter_C|GetAC_InventorySystem _ownercharacter))
  (bind _tools (Variables|/Script/ParkourPrototype.AC_InventorySystem|GetTools _ac_inventorysystem))
  (bind _output (Utilities|Array|Get(acopy) _tools))
  (bind (_itemname _itemclass _rarity _count _itemweight _description) (Utilities|Struct|BreakItems _output))
  (Utilities|IsValid _ac_inventorysystem_2
    (:Is%20Valid
      (bind _returnvalue (Class|ACInventorySystem|DecreaseItems _ac_inventorysystem_2 (Variables|Default|GetItemCost)))
      (if _returnvalue
        (|SetBy-RefVar _output (Utilities|Struct|MakeItems _itemname _itemclass _rarity (+ _count (Variables|Default|GetDoubleJumpCells)) _itemweight _description))
        (Default|UpdateText (Variables|/Game/FirstPersonBP/Blueprints/FirstPersonCharacter.FirstPersonCharacter_C|GetWDG_Inventory (Variables|Default|GetOwnerCharacter)))))))

(fn ConstructionScript)