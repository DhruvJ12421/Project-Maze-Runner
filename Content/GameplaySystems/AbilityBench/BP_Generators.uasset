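; BP_Generators is a generator in the Ability Bench system that shows its name, description and item cost on an in-world widget.
; On BeginPlay it caches the player character and WDG_Generator widget, then fills in the heading and text.
; GetCost builds the cost string by resolving each item's type and index against the player's inventory component.
; A looping timer toggles widget visibility from NearPlayer, which this graph never sets.
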(event Custom|NearVisibility
  ;[1 1 1] Near Player
  (Rendering|SetVisibility (Variables|Default|GetWDG_Generator) (Variables|Default|GetNearPlayer) false))

(event EventBeginPlay
  ;[1 1 1] Init
  (bind _asfirst_person_character (Utilities|Casting|CastToFirstPersonCharacter (Game|GetPlayerCharacter 0)))
  (Variables|Default|SetOwnerCharacter _asfirst_person_character)
  (bind _aswdg_generator (Utilities|Casting|CastToWDG_Generator (UserInterface|GetWidget (Variables|Default|GetWDG_Generator))))
  (Variables|Default|SetWDGGenerator _aswdg_generator)
  ;[1 1 1] Near Player
  (bind _returnvalue (Utilities|Time|SetTimerbyEvent (delegate Custom|NearVisibility) 0.1 true))
  (Variables|Default|SetTH_NearPlayer _returnvalue)
  ;[1 1 1] Widget Name
  (Default|UpdateHeading (Variables|Default|GetWDGGenerator) (Variables|Default|GetHeading%20Name))
  ;[1 1 1] WDG Description
  (Default|UpdateText (Variables|Default|GetWDGGenerator) (Utilities|Text|ToText(String) (Utilities|String|Append (Variables|Default|GetDescription) " 
 
" "Cost:-" " 
" (CallFunction|GetCost (Variables|Default|GetItemCost))))))

(fn ConstructionScript)

(fn GetCost
  (params (items :type Array%20of%20Decrease%20Item%20Structures))
  (bind _ownercharacter (Variables|Default|GetOwnerCharacter))
  (bind _ac_inventorysystem (Variables|/Game/FirstPersonBP/Blueprints/FirstPersonCharacter.FirstPersonCharacter_C|GetAC_InventorySystem _ownercharacter))
  (for (_array_element _array_index) items
    (if (== _array_index 0)
      (LocalVariables|SetRequiredString (Utilities|String|Append (Utilities|String|ToString(Name) (.ItemName (Utilities|Struct|BreakItems (Utilities|Array|Get(acopy) (Utilities|Select :Index (.Type (Utilities|Struct|BreakDecreaseItem _array_element)) :NONE 0 :Consumables (Variables|/Script/ParkourPrototype.AC_InventorySystem|GetConsumables _ac_inventorysystem) :Parts (Variables|/Script/ParkourPrototype.AC_InventorySystem|GetParts _ac_inventorysystem) :Materials (Variables|/Script/ParkourPrototype.AC_InventorySystem|GetMaterials _ac_inventorysystem) :Tools (Variables|/Script/ParkourPrototype.AC_InventorySystem|GetTools _ac_inventorysystem)) (.index (Utilities|Struct|BreakDecreaseItem _array_element)))))) " : " (Utilities|String|ToString(Integer) (.Amount (Utilities|Struct|BreakDecreaseItem _array_element)))))
      (else
        (LocalVariables|SetRequiredString (Utilities|String|Append (LocalVariables|GetRequiredString) " 
" (Utilities|String|Append (Utilities|String|ToString(Name) (.ItemName (Utilities|Struct|BreakItems (Utilities|Array|Get(acopy) (Utilities|Select :Index (.Type (Utilities|Struct|BreakDecreaseItem _array_element)) :NONE 0 :Consumables (Variables|/Script/ParkourPrototype.AC_InventorySystem|GetConsumables _ac_inventorysystem) :Parts (Variables|/Script/ParkourPrototype.AC_InventorySystem|GetParts _ac_inventorysystem) :Materials (Variables|/Script/ParkourPrototype.AC_InventorySystem|GetMaterials _ac_inventorysystem) :Tools (Variables|/Script/ParkourPrototype.AC_InventorySystem|GetTools _ac_inventorysystem)) (.index (Utilities|Struct|BreakDecreaseItem _array_element)))))) " : " (Utilities|String|ToString(Integer) (.Amount (Utilities|Struct|BreakDecreaseItem _array_element)))))))))
  (return (LocalVariables|GetRequiredString)))